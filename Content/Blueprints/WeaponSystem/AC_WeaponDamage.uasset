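; Weapon damage component that applies damage from firearm hits, reading damage settings from the owner's AC_WeaponSystem firearm description.
; Server single and multi-hit events apply flat base damage to blocking hits, crediting the owning Character's controller.
; A separate calculation scales damage by a distance-sampled curve and headshot-bone multiplier, but those events bypass it.
; Helpers also provide toggleable damage application with debug printing and trace-based hit-direction yaw.
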(event Custom|ServerHandleMultiHit
  (params (SingleHit :type Array%20of%20S%20Weapon%20Hit%20Scan%20Desc%20Structures))
  ;[1 1 1] HANDLE HIT
  ;;[1 1 1] Multi
  ;;;[1 0.1179 0] INPUT FROM FIREARM SYSTEM
  (for _array_element SingleHit
    (if (.BlockingHit (Utilities|Struct|BreakS_WeaponHitScanDesc _array_element))
      (bind _ascharacter (Utilities|Casting|CastToCharacter (Components|GetOwner)))
      (Game|Damage|ApplyDamage (.HitActor (Utilities|Struct|BreakS_WeaponHitScanDesc _array_element)) (GETFIREARMVALUES|GetDamageAmount) (Pawn|GetController _ascharacter) (Default|GetFirearmItemCommon (GETCOMPONENTS|GetFirearmSystem)) (GETFIREARMVALUES|GetDamageTypeClass)))))

(event Custom|ServerHandleSingleHit
  (params (SingleHit :type S%20Weapon%20Hit%20Scan%20Desc%20Structure))
  (bind (_blockinghit _distancetohit _tracestart _traceend _hitworldlocation _hitnormal _hitactor) (Utilities|Struct|BreakS_WeaponHitScanDesc SingleHit))
  ;[1 1 1] HANDLE HIT
  ;;[1 1 1] Single
  ;;;[1 0.1179 0] INPUT FROM FIREARM SYSTEM
  (if _blockinghit
    (bind _ascharacter (Utilities|Casting|CastToCharacter (Components|GetOwner)))
    (Game|Damage|ApplyDamage _hitactor (GETFIREARMVALUES|GetDamageAmount) (Pawn|GetController _ascharacter) (Default|GetFirearmItemCommon (GETCOMPONENTS|GetFirearmSystem)) (GETFIREARMVALUES|GetDamageTypeClass))))

(fn DamageCalculation
  (params (StartTracePoint :type Vector) (HitTracePoint :type Vector) (HitBoneName :type Name))
  (bind _damage_amount (GETFIREARMVALUES|GetDamageAmount))
  (bind (_x _y _z) (Math|Vector|BreakVector StartTracePoint))
  (bind _damage_coefficient (GETFIREARMVALUES|GetDamageCoefficient))
  (bind (_x_2 _y_2 _z_2) (Math|Vector|BreakVector HitTracePoint))
  (bind _shootingmaxdistance (Variables|SETTINGS|GetShootingMaxDistance))
  (bind _returnvalue (- _z_2 _z))
  (bind _returnvalue_2 (- _x_2 _x))
  (bind _returnvalue_3 (- _y_2 _y))
  (bind _returnvalue_4 (/ _shootingmaxdistance 1e+02))
  (bind _returnvalue_5 (Math|Float|Square _returnvalue))
  (bind _returnvalue_6 (Math|Float|Square _returnvalue_2))
  (bind _returnvalue_7 (Math|Float|Square _returnvalue_3))
  (bind _returnvalue_8 (+ _returnvalue_6 _returnvalue_7 _returnvalue_5))
  (bind _returnvalue_9 (Math|Float|Sqrt _returnvalue_8))
  (bind _returnvalue_10 (/ _returnvalue_9 _returnvalue_4))
  (bind _returnvalue_11 (/ _returnvalue_10 1e+02))
  (bind _returnvalue_12 (Math|Curves|GetFloatValue _damage_coefficient _returnvalue_11))
  (bind _returnvalue_13 (* _damage_amount _returnvalue_12))
  (Utilities|IsValid (GETFIREARMVALUES|GetDamageCoefficient)
    (:Is%20Valid
      (if (Utilities|Array|ContainsItem (Variables|SETTINGS|GetHead%20Shot%20Bones) HitBoneName)
        (LocalVariables|Setloc%20damage (* _returnvalue_13 (GETFIREARMVALUES|GetHeadshotMultiplier)))
        (else
          (LocalVariables|Setloc%20damage _returnvalue_13)))
      (return (LocalVariables|Getloc%20damage)))))

(fn GetDamageAmount
  (return (.DamageAmount (Utilities|Struct|BreakS_WeaponLibraryDamageDesc (.Damage (Utilities|Struct|BreakS_WeaponLibraryDesc (Default|GetFirearmLibraryDesc (GETCOMPONENTS|GetFirearmSystem))))))))

(fn GetDamageCoefficient
  (bind _firearmsystem (GETCOMPONENTS|GetFirearmSystem))
  (bind _firearmlibdesc (Default|GetFirearmLibraryDesc _firearmsystem))
  (bind _damage (Utilities|Struct|BreakS_WeaponLibraryDesc _firearmlibdesc))
  (bind _damagecoefficient (Utilities|Struct|BreakS_WeaponLibraryDamageDesc _damage))
  (Utilities|IsValid _damagecoefficient
    (:Is%20Valid
      (return _damagecoefficient))))

(fn GetHeadshotMultiplier
  (return (.HeadshotMultiplier (Utilities|Struct|BreakS_WeaponLibraryDamageDesc (.Damage (Utilities|Struct|BreakS_WeaponLibraryDesc (Default|GetFirearmLibraryDesc (GETCOMPONENTS|GetFirearmSystem))))))))

(fn GetDamageTypeClass
  (return (.DamageTypeClass (Utilities|Struct|BreakS_WeaponLibraryDamageDesc (.Damage (Utilities|Struct|BreakS_WeaponLibraryDesc (Default|GetFirearmLibraryDesc (GETCOMPONENTS|GetFirearmSystem))))))))

(fn GiveDamagetoHittedActor
  (params (DamagedActor :type Actor%20Object%20Reference) (Damage :type Float%20%28single-precision%29) (EventInstigator :type Controller%20Object%20Reference) (DamageCauser :type Actor%20Object%20Reference) (DamageTypeClass :type Damage%20Type%20Class%20Reference) (HitDirectionYaw :type Float%20%28double-precision%29))
  (if (not (Variables|SETTINGS|GetDamageOFF))
    (bind _returnvalue (Game|Damage|ApplyDamage DamagedActor Damage EventInstigator DamageCauser DamageTypeClass))
    (Development|PrintString (Utilities|String|ToString(Float) _returnvalue))))

(fn HitDirectionYawCalculation
  (params (StartTrace :type Vector) (EndTrace :type Vector))
  (bind _outhit (Collision|LineTraceForObjects StartTrace EndTrace (Utilities|Array|MakeArray "ObjectTypeQuery1" "ObjectTypeQuery7" "ObjectTypeQuery4" "ObjectTypeQuery5" "ObjectTypeQuery6") false (Utilities|Array|MakeArray (Components|GetOwner)) "None" true "(R=1.000000,G=0.000000,B=0.000000,A=1.000000)" "(R=0.000000,G=1.000000,B=0.000000,A=1.000000)" 0.5))
  (if (.bBlockingHit (Collision|BreakHitResult _outhit))
    (return (.Yaw (Math|Rotator|BreakRotator (Math|Rotator|MakeRotfromX (.Normal (Collision|BreakHitResult _outhit))))))))

(fn GetFirearmSystem
  (bind _self self)
  (bind _returnvalue (Components|GetOwner _self))
  (bind _returnvalue_2 (Actor|GetComponentbyClass _returnvalue "/Game/Blueprints/WeaponSystem/AC_WeaponSystem.AC_WeaponSystem_C"))
  (Utilities|IsValid _returnvalue_2
    (:Is%20Valid
      (return _returnvalue_2))))