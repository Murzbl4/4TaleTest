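; Client-side weapon component that turns fire and reload inputs into timed shot and reload events for the owner's AC_WeaponSystem.
; Automatic fire loops on a fire-rate timer; semi-auto adds a dense-compensation window for replaying buffered presses.
; Reloads, standard or cyclic (repeating until full or interrupted by firing), use retriggerable delays behind gates for cancellation.
; Tuning comes from the firearm library description, reserve ammo from AC_InventorySystem.
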(event Custom|ClientShootPressed
  ;[1 1 1] HANDLE INPUT PRESSED
  ;;[1 0.1179 0] INPUT FROM FIREARM SYSTEM
  ;;[0 1 0.2254] InputFireHold = True
  (Variables|COMMON|SetInputFireHold true)
  ;;[0 0.3159 1] CONDITION: InMainReload = true or InExtraReload = true
  (if (or (Variables|COMMON|GetInMainReload) (Variables|COMMON|GetInExtraReload))
    ;;[0 0.3159 1] CONDITION: GetCyclicMainReload = True and InMainReload = true
    (if (and (GETFIREARMVALUES|GetCyclicMainReload) (Variables|COMMON|GetInMainReload))
      ;;[0 1 0.2254] RequestForCancelCyclicMainReload = true
      (Variables|COMMON|SetRequestForCancelCyclicMainReload true))
    (else
      ;;[0 0.3159 1] CONDITION: GetCurrentClipSize = 0
      (if (== (GETFIREARMVALUES|GetCurrentClipSize) 0)
        ;;[0 0.3159 1] CONDITION: GetCurrentAmmoPull = 0
        (if (== (GETFIREARMVALUES|GetCurrentAmmoPull) 0)
          ;;[1 0 0.008047] TRIGGER: ClientFirearmsAmmoEmpty
          (CallFunction|ClientFirearmsAmmoEmpty)
          (else
            ;;[1 0 0.008047] TRIGGER: ClientRequestedMainReload
            (CallFunction|ClientRequestedMainReload)))
        (else
          ;;[0 0.3159 1] CONDITION: WaitShotDelay = true
          (if (not (Variables|COMMON|GetWaitShotDelay))
            ;;[0 0.3159 1] CONDITION: FiringMode
            (switch Utilities|FlowControl|Switch|SwitchonE_GL_WeaponFiringMode (GETFIREARMVALUES|GetFiringMode)
              (:NewEnumerator0
                ;;[1 0 0.008047] TRIGGER: ClientCreateShot
                (CallFunction|ClientCreateShot)
                ;;[1 0 0.008047] TRIGGER TIMER: ClientCreateShot
                (Utilities|Time|SetTimerbyFunctionName 0 "ClientCreateShot" (GETFIREARMVALUES|GetShotDelay) true))
              (:NewEnumerator1
                ;;[1 0 0.008047] TRIGGER: ClientCreateShot
                (CallFunction|ClientCreateShot)))))))))

(event Custom|ClientShootReleased
  ;[1 1 1] HANDLE INPUT RELEASED  & OTHERS
  ;;[1 0.1179 0] INPUT FROM FIREARM SYSTEM
  (Variables|COMMON|SetInputFireHold false)
  (switch Utilities|FlowControl|Switch|SwitchonE_GL_WeaponFiringMode (GETFIREARMVALUES|GetFiringMode)
    (:NewEnumerator0
      (Utilities|Time|ClearTimerbyFunctionName 0 "ClientCreateShot"))))

(event Custom|ClientTriggerNewCyclicMainReload
  ;[1 1 1] OUTPUTS & RELOAD
  ;;[1 1 1] Cyclic Main Reload
  ;;;[1 1 1] Cyclic Main reload time
  ;;;;[0.9739 1 0] BI OUTPUT TO FirearmSystem
  (Default|ClientMainReloadCyclicStart (GETCOMPONENTS|GetFirearmSystem))
  (Utilities|FlowControl|Sequence
    (:then_0
      (Utilities|FlowControl|RetriggerableDelay (GETFIREARMVALUES|GetMainReloadTime))
      (Utilities|FlowControl|Gate false :!label _label
        (:Exit
          ;;;;[0.9739 1 0] BI OUTPUT TO FirearmSystem
          (Default|ClientMainReloadCyclicStop (GETCOMPONENTS|GetFirearmSystem))
          ;;;[1 1 1] Check condition to finish cyclic main reload
          (if (== (GETFIREARMVALUES|GetCurrentClipSize) (GETFIREARMVALUES|GetClipSize))
            ;;;[1 1 1] Transfer to default pos
            ;;;;[0.9739 1 0] BI OUTPUT TO FirearmSystem
            (Default|ClientMainReloadCyclicEndtoPos (GETCOMPONENTS|GetFirearmSystem) :!label _label_2)
            (Utilities|FlowControl|Sequence
              (:then_0
                (Utilities|FlowControl|RetriggerableDelay (GETFIREARMVALUES|GetCyclicMainReloadEndingTime))
                (Utilities|FlowControl|Gate false :!label _label_3
                  (:Exit
                    ;;;;[0.9739 1 0] BI OUTPUT TO FirearmSystem
                    (Default|ClientMainReloadStart (GETCOMPONENTS|GetFirearmSystem))
                    (Variables|COMMON|SetInMainReload false))))
              (:then_1
                (goto _label_3 Open)))
            (else
              ;;;[1 1 1] Check Input storing in main reload state by input pressed
              (if (Variables|COMMON|GetRequestForCancelCyclicMainReload)
                (Variables|COMMON|SetRequestForCancelCyclicMainReload false)
                (goto _label_2)
                (else
                  (CallFunction|ClientTriggerNewCyclicMainReload))))))))
    (:then_1
      (goto _label Open))))

(event Custom|ClientResetGateMainReload
  ;[1 1 1] OUTPUTS & RELOAD
  ;;[1 1 1] Main Reload
  (Utilities|FlowControl|DoOnce false) ; enters at Reset
)

(event Custom|ClientSetBlockAnyAction
  (params (InBlockAnyAction :type Boolean))
  ;[1 1 1] HANDLE INPUT RELEASED  & OTHERS
  ;;[1 0.1179 0] INPUT FROM FIREARM SYSTEM
  (bind _output_get (Variables|COMMON|SetInBlockAnyAction InBlockAnyAction))
  (if _output_get
    (CallFunction|ClientCancelMainReload)
    (CallFunction|ClientCancelCyclicMainReload)))

(event Custom|ClientCancelMainReload
  ;[1 1 1] OUTPUTS & RELOAD
  ;;[1 1 1] Main Reload
  ;;;[1 1 1] Main reload delay logic
  ;;;;[0.9739 1 0] BI OUTPUT TO FirearmSystem
  (Default|ClientMainReloadCanceled (GETCOMPONENTS|GetFirearmSystem))
  (Utilities|FlowControl|Gate false) ; enters at Close
)

(event Custom|ClientCreateShot
  ;[1 1 1] CREATE SHOT
  ;;[0.2033 0.3085 1] LOCAL INPUT
  ;;[0 0.3159 1] CONDITION: GetCurrentClipSize = 0
  (if (== (GETFIREARMVALUES|GetCurrentClipSize) 0)
    ;;[0 0.3159 1] CONDITION: GetCurrentAmmoPull = 0
    (if (== (GETFIREARMVALUES|GetCurrentAmmoPull) 0)
      ;;[1 0 0.008047] TRIGGER: ClientFirearmsAmmoEmpty
      (CallFunction|ClientFirearmsAmmoEmpty)
      (else
        (CallFunction|ClientRequestedMainReload)))
    (else
      ;;[0 1 0.2254] WaitShotDelay = true
      (Variables|COMMON|SetWaitShotDelay true)
      ;;[1 0 0.008047] TRIGGER: ClientShotHappened
      (CallFunction|ClientShotHappened)
      ;;[0 0.3159 1] SEQUENCE
      (Utilities|FlowControl|Sequence
        (:then_0
          (Utilities|FlowControl|Sequence
            (:then_0
              (Utilities|FlowControl|Delay (GETFIREARMVALUES|GetShotDelay))
              (Variables|COMMON|SetWaitShotDelay false)
              (Variables|COMMON|SetCanUseDenseComp false)
              ;;[1 0 0.008047] TRIGGER: ClientShotDelayEnded
              (CallFunction|ClientShotDelayEnded)
              ;;[1 1 1] End shot logic
              ;;;[1 1 1] Check request for main reload
              (if (Variables|COMMON|GetRequestForMainReload)
                (Variables|COMMON|SetRequestForMainReload false)
                (CallFunction|ClientRequestedMainReload)
                (else
                  ;;;[1 1 1] Check clip == 0
                  (if (== (GETFIREARMVALUES|GetCurrentClipSize) 0)
                    (CallFunction|ClientRequestedMainReload)
                    (else
                      ;;;[1 1 1] Handle DenseComp after shot delay
                      (if (Variables|COMMON|GetDenseCompInputStoring)
                        (CallFunction|ClientShootPressed)
                        (Variables|COMMON|SetDenseCompInputStoring false)))))))
            (:then_1
              (if (Utilities|Enum|Equal(Enum) (GETFIREARMVALUES|GetFiringMode) "NewEnumerator1")
                ;;[1 1 1] Calculation time in shot delay period when dense compensation windows is closed
                (Utilities|FlowControl|Delay (* (GETFIREARMVALUES|GetDenseCompensation) (GETFIREARMVALUES|GetShotDelay)))
                (Variables|COMMON|SetCanUseDenseComp true)))))))))

(event Custom|ClientShotHappened
  ;[1 1 1] OUTPUTS & RELOAD
  ;;[1 1 1] Shot & Ammo is empty
  ;;;[0.9739 1 0] BI OUTPUT TO FirearmSystem
  (Default|ClientShotHappened (GETCOMPONENTS|GetFirearmSystem)))

(event Custom|ClientShotDelayEnded
  ;[1 1 1] OUTPUTS & RELOAD
  ;;[1 1 1] Shot & Ammo is empty
  ;;;[0.9739 1 0] BI OUTPUT TO FirearmSystem
  (Default|ClientShotDelayEnded (GETCOMPONENTS|GetFirearmSystem)))

(event Custom|ClientFirearmsAmmoEmpty
  ;[1 1 1] OUTPUTS & RELOAD
  ;;[1 1 1] Shot & Ammo is empty
  (Utilities|Time|ClearTimerbyFunctionName 0 "ClientCreateShot")
  ;;;[0.9739 1 0] BI OUTPUT TO FirearmSystem
  (Default|ClientFirearmsAmmoEmpty (GETCOMPONENTS|GetFirearmSystem)))

(event Custom|ClientRequestedMainReload
  ;[1 1 1] OUTPUTS & RELOAD
  ;;[1 1 1] Main Reload
  ;;;[1 0.1179 0] INPUT FROM FIREARM SYSTEM
  (Utilities|FlowControl|DoOnce false
    (:Completed
      (Utilities|FlowControl|Delay 0.2)
      (CallFunction|ClientResetGateMainReload)
      (if (not (Variables|COMMON|GetInBlockAnyAction))
        ;;;[1 1 1] Check clip = full
        (if (not (== (GETFIREARMVALUES|GetClipSize) (GETFIREARMVALUES|GetCurrentClipSize)))
          ;;;[1 1 1] Main reload conditions
          (if (Math|Boolean|ANDBoolean (not (Variables|COMMON|GetInMainReload)) (not (== (GETFIREARMVALUES|GetCurrentAmmoPull) 0)) (not (Variables|COMMON|GetInBlockAnyAction)))
            (Variables|COMMON|SetDenseCompInputStoring false)
            ;;;[1 1 1] Handle Weapon types
            (switch Utilities|FlowControl|Switch|SwitchonE_GL_WeaponFiringMode (GETFIREARMVALUES|GetFiringMode)
              (:NewEnumerator0
                (Utilities|Time|ClearTimerbyFunctionName 0 "ClientCreateShot")
                ;;;[1 1 1] Check CylclicMainReload Principal.
                (if (GETFIREARMVALUES|GetCyclicMainReload) :!label _label
                  (CallFunction|ClientHandleCyclicMainReload)
                  (else
                    (Variables|COMMON|SetInMainReload true)
                    ;;;[1 1 1] Main reload delay logic
                    ;;;;[0.9739 1 0] BI OUTPUT TO FirearmSystem
                    (Default|ClientMainReloadStart (GETCOMPONENTS|GetFirearmSystem))
                    (Utilities|FlowControl|Sequence
                      (:then_0
                        (Utilities|FlowControl|RetriggerableDelay (GETFIREARMVALUES|GetMainReloadTime))
                        (Utilities|FlowControl|Gate false :!label _label_2
                          (:Exit
                            ;;;;[0.9739 1 0] BI OUTPUT TO FirearmSystem
                            (Default|ClientMainReloadFinish (GETCOMPONENTS|GetFirearmSystem))
                            (Variables|COMMON|SetInMainReload false)
                            ;;;[1 1 1] Triggers shooting after main reload if input fire is holded
                            (if (Variables|COMMON|GetInputFireHold)
                              (CallFunction|ClientShootPressed)))))
                      (:then_1
                        (goto _label_2 Open))))))
              (:NewEnumerator1
                (if (Variables|COMMON|GetWaitShotDelay)
                  (Variables|COMMON|SetRequestForMainReload true)
                  (else
                    (goto _label)))))))))))

(event Custom|ClientHandleCyclicMainReload
  ;[1 1 1] OUTPUTS & RELOAD
  ;;[1 1 1] Cyclic Main Reload
  (Variables|COMMON|SetInMainReload true)
  ;;;[1 1 1] Starting
  ;;;;[0.9739 1 0] BI OUTPUT TO FirearmSystem
  (Default|ClientMainReloadCyclicStarttoPos (GETCOMPONENTS|GetFirearmSystem))
  (Utilities|FlowControl|Sequence
    (:then_0
      (Utilities|FlowControl|RetriggerableDelay (GETFIREARMVALUES|GetCyclicMainReloadStartingTime))
      (Utilities|FlowControl|Gate false :!label _label
        (:Exit
          ;;;[1 1 1] Cyclic Main reload time
          ;;;;[0.9739 1 0] BI OUTPUT TO FirearmSystem
          (Default|ClientMainReloadCyclicStart (GETCOMPONENTS|GetFirearmSystem))
          (Utilities|FlowControl|Sequence
            (:then_0
              (Utilities|FlowControl|RetriggerableDelay (GETFIREARMVALUES|GetMainReloadTime))
              (Utilities|FlowControl|Gate false :!label _label_2
                (:Exit
                  ;;;;[0.9739 1 0] BI OUTPUT TO FirearmSystem
                  (Default|ClientMainReloadCyclicStop (GETCOMPONENTS|GetFirearmSystem))
                  ;;;[1 1 1] Check condition to finish cyclic main reload
                  (if (== (GETFIREARMVALUES|GetCurrentClipSize) (GETFIREARMVALUES|GetClipSize))
                    ;;;[1 1 1] Transfer to default pos
                    ;;;;[0.9739 1 0] BI OUTPUT TO FirearmSystem
                    (Default|ClientMainReloadCyclicEndtoPos (GETCOMPONENTS|GetFirearmSystem) :!label _label_3)
                    (Utilities|FlowControl|Sequence
                      (:then_0
                        (Utilities|FlowControl|RetriggerableDelay (GETFIREARMVALUES|GetCyclicMainReloadEndingTime))
                        (Utilities|FlowControl|Gate false :!label _label_4
                          (:Exit
                            ;;;;[0.9739 1 0] BI OUTPUT TO FirearmSystem
                            (Default|ClientMainReloadStart (GETCOMPONENTS|GetFirearmSystem))
                            (Variables|COMMON|SetInMainReload false))))
                      (:then_1
                        (goto _label_4 Open)))
                    (else
                      ;;;[1 1 1] Check Input storing in main reload state by input pressed
                      (if (Variables|COMMON|GetRequestForCancelCyclicMainReload)
                        (Variables|COMMON|SetRequestForCancelCyclicMainReload false)
                        (goto _label_3)
                        (else
                          (CallFunction|ClientTriggerNewCyclicMainReload))))))))
            (:then_1
              (goto _label_2 Open))))))
    (:then_1
      (goto _label Open))))

(event Custom|ClientCancelCyclicMainReload
  ;[1 1 1] OUTPUTS & RELOAD
  ;;[1 1 1] Cyclic Main Reload
  ;;;[1 1 1] Starting
  ;;;;[0.9739 1 0] BI OUTPUT TO FirearmSystem
  (Default|ClientMainReloadCanceled (GETCOMPONENTS|GetFirearmSystem))
  (Utilities|FlowControl|Sequence
    (:then_0
      (Utilities|FlowControl|Gate false) ; enters at Close
    )
    (:then_1
      ;;;[1 1 1] Cyclic Main reload time
      ;;;;[0.9739 1 0] BI OUTPUT TO FirearmSystem
      (Default|ClientMainReloadCanceled (GETCOMPONENTS|GetFirearmSystem))
      (Utilities|FlowControl|Sequence
        (:then_0
          (Utilities|FlowControl|Gate false) ; enters at Close
        )
        (:then_1
          ;;;[1 1 1] Transfer to default pos
          ;;;;[0.9739 1 0] BI OUTPUT TO FirearmSystem
          (Default|ClientMainReloadCanceled (GETCOMPONENTS|GetFirearmSystem))
          (Utilities|FlowControl|Gate false) ; enters at Close
        )))))

(fn GetFirearmSystem
  (bind _returnvalue (Components|GetOwner))
  (bind _returnvalue_2 (Actor|GetComponentbyClass _returnvalue "/Game/Blueprints/WeaponSystem/AC_WeaponSystem.AC_WeaponSystem_C"))
  (Utilities|IsValid _returnvalue_2
    (:Is%20Valid
      (return _returnvalue_2))))

(fn GetFiringMode
  (return (.FiringMode (Utilities|Struct|BreakS_WeaponLibraryShootDesc (.Shoot (Utilities|Struct|BreakS_WeaponLibraryDesc (Default|GetFirearmLibraryDesc (GETCOMPONENTS|GetFirearmSystem))))))))

(fn GetCyclicMainReload
  (return (.CyclicMainReload (Utilities|Struct|BreakS_WeaponLibraryCommonDesc (.Common (Utilities|Struct|BreakS_WeaponLibraryDesc (Default|GetFirearmLibraryDesc (GETCOMPONENTS|GetFirearmSystem))))))))

(fn GetCurrentAmmoPull
  (LocalVariables|Setloc_ammo_type (.AmmoType (Utilities|Struct|BreakS_WeaponLibraryAmmoDesc (.AmmoClip (Utilities|Struct|BreakS_WeaponLibraryDesc (Default|GetFirearmLibraryDesc (GETCOMPONENTS|GetFirearmSystem)))))))
  (for _array_element (Default|GetInventoryResources (GETCOMPONENTS|GetInventorySystem))
    (LocalVariables|Setloc_res_type (.ResourceType (Utilities|Struct|BreakS_GL_InventoryResourceDesc _array_element)))
    (LocalVariables|Setloc_spet_ammo (.Amount (Utilities|Struct|BreakS_GL_InventoryResourceDesc _array_element)))
    (switch Utilities|FlowControl|Switch|SwitchonE_WeaponAmmoType (LocalVariables|Getloc_ammo_type)
      (:NewEnumerator0
        (if (Utilities|Enum|Equal(Enum) (LocalVariables|Getloc_res_type) "NewEnumerator0")
          (LocalVariables|Setloc_ammo_res_current (LocalVariables|Getloc_spet_ammo))))
      (:NewEnumerator1
        (if (Utilities|Enum|Equal(Enum) (LocalVariables|Getloc_res_type) "NewEnumerator1")
          (LocalVariables|Setloc_ammo_res_current (LocalVariables|Getloc_spet_ammo))))))
  (return (LocalVariables|Getloc_ammo_res_current)))

(fn GetCurrentClipSize
  (Utilities|IsValid (Default|GetFirearmItemCommon (GETCOMPONENTS|GetFirearmSystem))
    (:Is%20Valid
      (return (Default|GetCurrentAmmoinClip (Default|GetFirearmItemCommon (GETCOMPONENTS|GetFirearmSystem)))))))

(fn GetShotDelay
  (return (/ 1.0 (/ (Math|Conversions|ToFloat(Integer) (.FireRate (Utilities|Struct|BreakS_WeaponLibraryShootDesc (.Shoot (Utilities|Struct|BreakS_WeaponLibraryDesc (Default|GetFirearmLibraryDesc (GETCOMPONENTS|GetFirearmSystem))))))) 6e+01))))

(fn GetBurstFireShotsBeforePause
  (return (.BurstFireShotsBeforePause (Utilities|Struct|BreakS_WeaponLibraryShootDesc (.Shoot (Utilities|Struct|BreakS_WeaponLibraryDesc (Default|GetFirearmLibraryDesc (GETCOMPONENTS|GetFirearmSystem))))))))

(fn GetBurstFirePause
  (return (.BurstFirePause (Utilities|Struct|BreakS_WeaponLibraryShootDesc (.Shoot (Utilities|Struct|BreakS_WeaponLibraryDesc (Default|GetFirearmLibraryDesc (GETCOMPONENTS|GetFirearmSystem))))))))

(fn GetDenseCompensation
  (return (.DenseCompensation (Utilities|Struct|BreakS_WeaponLibraryShootDesc (.Shoot (Utilities|Struct|BreakS_WeaponLibraryDesc (Default|GetFirearmLibraryDesc (GETCOMPONENTS|GetFirearmSystem))))))))

(fn GetShotTimePart
  (return (.ShotTimePart (Utilities|Struct|BreakS_WeaponLibraryShootDesc (.Shoot (Utilities|Struct|BreakS_WeaponLibraryDesc (Default|GetFirearmLibraryDesc (GETCOMPONENTS|GetFirearmSystem))))))))

(fn GetClipSize
  (return (Utilities|Struct|BreakS_WeaponLibraryAmmoDesc (Utilities|Struct|BreakS_WeaponLibraryDesc (Default|GetFirearmLibraryDesc (GETCOMPONENTS|GetFirearmSystem))))))

(fn GetMainReloadTime
  (return (.MainReloadTime (Utilities|Struct|BreakS_WeaponLibraryActionDesc (.Action (Utilities|Struct|BreakS_WeaponLibraryDesc (Default|GetFirearmLibraryDesc (GETCOMPONENTS|GetFirearmSystem))))))))

(fn GetCyclicMainReloadStartingTime
  (return (.CyclicMainReloadStartingTime (Utilities|Struct|BreakS_WeaponLibraryActionDesc (.Action (Utilities|Struct|BreakS_WeaponLibraryDesc (Default|GetFirearmLibraryDesc (GETCOMPONENTS|GetFirearmSystem))))))))

(fn GetCyclicMainReloadEndingTime
  (return (.CyclicMainReloadEndingTime (Utilities|Struct|BreakS_WeaponLibraryActionDesc (.Action (Utilities|Struct|BreakS_WeaponLibraryDesc (Default|GetFirearmLibraryDesc (GETCOMPONENTS|GetFirearmSystem))))))))

(fn GetInventorySystem
  (bind _returnvalue (Components|GetOwner))
  (bind _returnvalue_2 (Actor|GetComponentbyClass _returnvalue "/Game/Blueprints/InventorySystem/AC_InventorySystem.AC_InventorySystem_C"))
  (Utilities|IsValid _returnvalue_2
    (:Is%20Valid
      (return _returnvalue_2))))