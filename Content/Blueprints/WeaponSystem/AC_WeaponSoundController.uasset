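; Actor component that plays firearm audio for shots, shell drops, surface impacts, zoom, weapon switching and reload actions.
; It handles calls from the firearm system and reads cues from the firearm library description of the owner's AC_WeaponSystem.
; Shot and hit sounds go through server-to-multicast events as 3D audio, with multi-hits sounding one random hit.
; Zoom, switch and reload sounds play in 2D, while shell drops use a delayed owner-only 3D sound.
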(event Custom|ClientPlayZoomInSound
  ;[1 1 1] ZOOM IN / OUT
  ;;[1 0.1179 0] BI INPUT FROM FIREARM SYSTEM
  (Audio|PlaySound2D (GETFIREARMVALUES|GetZoominSound) (Variables|Settings|GetWeapon%20Sound%20Volume%20Multiplier) 1.0 0.0 0 0))

(event Custom|ClientHandlePlayerSoundOnShot
  (bind _firearmsystem (GETCOMPONENTS|GetFirearmSystem))
  (bind _firearmitemcommon (Default|GetFirearmItemCommon _firearmsystem))
  (bind _returnvalue (Transformation|GetActorLocation _firearmitemcommon))
  ;[1 1 1] ON SHOT
  ;;[1 0.1179 0] BI INPUT FROM FIREARM SYSTEM
  (CallFunction|ServerHandlePlayerSoundonShot _returnvalue)
  ;;[1 1 1] Shell drop fake delay. Because we want that shell drop sound works for owner only
  (Utilities|FlowControl|Delay 0.5)
  (CallFunction|ClientPlayShellDropSound _returnvalue))

(event Custom|MulticastPlayerHitSoundAtLocation
  (params (HitLocation :type Vector) (SurfaceType :type EPhysicalSurface%20Enum :default "SurfaceType_Default"))
  ;[1 1 1] ON HIT
  (COMMON|PlayHitPointSound HitLocation SurfaceType))

(event Custom|ClientHandleAnimEventReloadAction
  (params (Index :type Integer))
  ;[1 1 1] ON RELOAD ACTION
  ;;[1 0.1179 0] BI INPUT FROM FIREARM SYSTEM
  (for _array_element (GETFIREARMVALUES|GetReloadActionSoundes)
    (if (== (.Index (Utilities|Struct|BreakS_WeaponActionSoundDesc _array_element)) Index)
      (Variables|COMMON|SetReloadActionSound (.SoundCue (Utilities|Struct|BreakS_WeaponActionSoundDesc _array_element)))))
  (Audio|PlaySound2D (Variables|COMMON|GetReloadActionSound) (Variables|Settings|GetWeapon%20Sound%20Volume%20Multiplier) 1.0 0.0 0 0))

(event Custom|ClientPlaySwitchUpSound
  ;[1 1 1] SWITCH DOWN / UP
  ;;[1 0.1179 0] BI INPUT FROM FIREARM SYSTEM
  (Audio|PlaySound2D (GETFIREARMVALUES|GetSwitchUp) (Variables|Settings|GetWeapon%20Sound%20Volume%20Multiplier) 1.0 0.0 0 0))

(event Custom|ServerHandlePlayerSoundOnShot
  (params (Location :type Vector))
  ;[1 1 1] ON SHOT
  (CallFunction|MulticastPlayShotSound Location))

(event Custom|ClientPlayShellDropSound
  (params (Location :type Vector))
  ;[1 1 1] ON SHOT
  (Utilities|FlowControl|Delay 0.05)
  (COMMON|Play3DSoundatLocation (GETFIREARMVALUES|GetShellFallSound) Location))

(event Custom|MulticastPlayShotSound
  (params (Location :type Vector))
  ;[1 1 1] ON SHOT
  (COMMON|Play3DSoundatLocation (GETFIREARMVALUES|GetWeaponShotSoundCue) Location))

(event Custom|ClientPlayZoomOutSound
  ;[1 1 1] ZOOM IN / OUT
  ;;[1 0.1179 0] BI INPUT FROM FIREARM SYSTEM
  (Audio|PlaySound2D (GETFIREARMVALUES|GetZoomOutSound) (Variables|Settings|GetWeapon%20Sound%20Volume%20Multiplier) 1.0 0.0 0 0))

(event Custom|ClientHandlePlayerSoundOnMultiHit
  (params (SingleHit :type Array%20of%20S%20Weapon%20Hit%20Scan%20Desc%20Structures))
  (bind _outitem (Utilities|Array|Random SingleHit))
  (bind (_blockinghit _distancetohit _tracestart _traceend _hitworldlocation _hitnormal _hitactor _hitbonename _hitsurface) (Utilities|Struct|BreakS_WeaponHitScanDesc _outitem))
  ;[1 1 1] ON HIT
  ;;[1 0.1179 0] BI INPUT FROM FIREARM SYSTEM
  (if _blockinghit
    (CallFunction|ServerPlayerHitSoundatLocation _hitworldlocation _hitsurface)))

(event Custom|ClientHandlePlayerSoundOnSingleHit
  (params (SingleHit :type S%20Weapon%20Hit%20Scan%20Desc%20Structure))
  (bind (_blockinghit _distancetohit _tracestart _traceend _hitworldlocation _hitnormal _hitactor _hitbonename _hitsurface) (Utilities|Struct|BreakS_WeaponHitScanDesc SingleHit))
  ;[1 1 1] ON HIT
  ;;[1 0.1179 0] BI INPUT FROM FIREARM SYSTEM
  (if _blockinghit
    (CallFunction|ServerPlayerHitSoundatLocation _hitworldlocation _hitsurface)))

(event Custom|ClientPlaySwitchDownSound
  ;[1 1 1] SWITCH DOWN / UP
  ;;[1 0.1179 0] BI INPUT FROM FIREARM SYSTEM
  (Audio|PlaySound2D (GETFIREARMVALUES|GetSwitchDown) (Variables|Settings|GetWeapon%20Sound%20Volume%20Multiplier) 1.0 0.0 0 0))

(event Custom|ServerPlayerHitSoundAtLocation
  (params (HitLocation :type Vector) (SurfaceType :type EPhysicalSurface%20Enum :default "SurfaceType_Default"))
  ;[1 1 1] ON HIT
  (CallFunction|MulticastPlayerHitSoundatLocation HitLocation SurfaceType))

(fn GetWeaponShotSoundCue
  (return (.WeaponShotSoundCue (Utilities|Struct|BreakS_FL_WeaponLibrarySoundDesc (.Sound (Utilities|Struct|BreakS_WeaponLibraryDesc (Default|GetFirearmLibraryDesc (GETCOMPONENTS|GetFirearmSystem))))))))

(fn Play3DSoundatLocation
  (params (Sound :type Sound%20Base%20Object%20Reference) (Location :type Vector))
  (Utilities|IsValid Sound
    (:Is%20Valid
      (Audio|PlaySoundatLocation Sound Location "0, 0, 0" (Variables|Settings|GetWeapon%20Sound%20Volume%20Multiplier) 1.0 0.0 0 0 0 0))))

(fn GetShellFallSound
  (return (.ShellFallSound (Utilities|Struct|BreakS_FL_WeaponLibrarySoundDesc (.Sound (Utilities|Struct|BreakS_WeaponLibraryDesc (Default|GetFirearmLibraryDesc (GETCOMPONENTS|GetFirearmSystem))))))))

(fn GetSurfaceHitSoundCueArray
  (return (.SurfaceHitSoundCueArray (Utilities|Struct|BreakS_FL_WeaponLibrarySoundDesc (.Sound (Utilities|Struct|BreakS_WeaponLibraryDesc (Default|GetFirearmLibraryDesc (GETCOMPONENTS|GetFirearmSystem))))))))

(fn GetReloadActionSoundes
  (return (.ReloadActionSoundes (Utilities|Struct|BreakS_FL_WeaponLibrarySoundDesc (.Sound (Utilities|Struct|BreakS_WeaponLibraryDesc (Default|GetFirearmLibraryDesc (GETCOMPONENTS|GetFirearmSystem))))))))

(fn PlayHitPointSound
  (params (Location :type Vector) (SurfaceType :type EPhysicalSurface%20Enum :default "SurfaceType_Default"))
  ;[1 1 1] hit sound
  (for _array_element (GETFIREARMVALUES|GetSurfaceHitSoundCueArray)
    (if (Utilities|Enum|Equal(Enum) (.Surface (Utilities|Struct|BreakS_SoundBaseonSurfaceDesc _array_element)) SurfaceType)
      (LocalVariables|Setloc_hit_sound (.SoundCUE (Utilities|Struct|BreakS_SoundBaseonSurfaceDesc _array_element)))))
  (Audio|PlaySoundatLocation (LocalVariables|Getloc_hit_sound) Location "0, 0, 0" (Variables|Settings|GetWeapon%20Sound%20Volume%20Multiplier) 1.0 0.0 0 0 0 0))

(fn GetFirearmSystem
  (bind _self self)
  (bind _returnvalue (Components|GetOwner _self))
  (bind _returnvalue_2 (Actor|GetComponentbyClass _returnvalue "/Game/Blueprints/WeaponSystem/AC_WeaponSystem.AC_WeaponSystem_C"))
  (Utilities|IsValid _returnvalue_2
    (:Is%20Valid
      (return _returnvalue_2))))

(fn GetZoominSound
  (return (.ZoomInSound (Utilities|Struct|BreakS_FL_WeaponLibrarySoundDesc (.Sound (Utilities|Struct|BreakS_WeaponLibraryDesc (Default|GetFirearmLibraryDesc (GETCOMPONENTS|GetFirearmSystem))))))))

(fn GetZoomOutSound
  (return (.ZoomOutSound (Utilities|Struct|BreakS_FL_WeaponLibrarySoundDesc (.Sound (Utilities|Struct|BreakS_WeaponLibraryDesc (Default|GetFirearmLibraryDesc (GETCOMPONENTS|GetFirearmSystem))))))))

(fn GetSwitchDown
  (return (.SwitchDown (Utilities|Struct|BreakS_FL_WeaponLibrarySoundDesc (.Sound (Utilities|Struct|BreakS_WeaponLibraryDesc (Default|GetFirearmLibraryDesc (GETCOMPONENTS|GetFirearmSystem))))))))

(fn GetSwitchUp
  (return (.SwitchUp (Utilities|Struct|BreakS_FL_WeaponLibrarySoundDesc (.Sound (Utilities|Struct|BreakS_WeaponLibraryDesc (Default|GetFirearmLibraryDesc (GETCOMPONENTS|GetFirearmSystem))))))))