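; Weapon VFX controller component that spawns replicated bullet impact effects and decals for its owner's firearm.
; Client events take single or multi hit-scan results and send each to a server event, which multicasts blocking hits.
; Each impact picks a particle and fading decal by surface type from the sibling AC_WeaponSystem's firearm library data, oriented to the hit normal.
; Scope and first-person inputs are stored, but do not affect the spawned effects.
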(event Custom|ClientStartPlayVFXOnCreateSingleHitScanTP
  (params (SingleHitScan :type S%20Weapon%20Hit%20Scan%20Desc%20Structure) (TPFirearmMesh :type Skeletal%20Mesh%20Component%20Object%20Reference) (WithHideForOwner :type Boolean))
  (bind (_blockinghit _distancetohit _tracestart _traceend _hitworldlocation _hitnormal _hitactor _hitbonename _hitsurface) (Utilities|Struct|BreakS_WeaponHitScanDesc SingleHitScan))
  ;[1 1 1] ON CREATE HIT SCAN
  ;;[1 1 1] TP / Single Trace
  ;;;[1 0.1179 0] INPUT FROM CHARACTER TP / FP
  (CallFunction|ServerCreateHitPointVFX _blockinghit _hitworldlocation _hitnormal _hitsurface)
  (if (Variables|State|GetInFPMode)
    (Variables|State|SetWithHideForOwner WithHideForOwner)
    (else
      (Variables|State|SetWithHideForOwner false))))

(event Custom|ClientStartPlayVFXOnCreateMultiHitScanTP
  (params (MultiHitScan :type Array%20of%20S%20Weapon%20Hit%20Scan%20Desc%20Structures) (TPFirearmMesh :type Skeletal%20Mesh%20Component%20Object%20Reference) (WithHideForOwner :type Boolean))
  ;[1 1 1] ON CREATE HIT SCAN
  ;;[1 1 1] TP / Multi Trace
  ;;;[1 0.1179 0] INPUT FROM CHARACTER TP / FP
  (for _array_element MultiHitScan
    (CallFunction|ServerCreateHitPointVFX (.BlockingHit (Utilities|Struct|BreakS_WeaponHitScanDesc _array_element)) (.HitWorldLocation (Utilities|Struct|BreakS_WeaponHitScanDesc _array_element)) (.HitNormal (Utilities|Struct|BreakS_WeaponHitScanDesc _array_element)) (.HitSurface (Utilities|Struct|BreakS_WeaponHitScanDesc _array_element)))
    (if (Variables|State|GetInFPMode)
      (Variables|State|SetWithHideForOwner WithHideForOwner)
      (else
        (Variables|State|SetWithHideForOwner false)))))

(event Custom|MulticastCreateHitPointVFX
  (params (HitPointLocation :type Vector) (HitPointNormal :type Vector) (SurfaceType :type EPhysicalSurface%20Enum :default "SurfaceType_Default"))
  ;[1 1 1] HIT POINT VFX
  ;;[1 1 1] MulticastCreateHitPointVFX
  (COMMON|CreateHitPointVFX HitPointLocation HitPointNormal SurfaceType)
  (COMMON|CreateHitPointDecal HitPointLocation HitPointNormal SurfaceType))

(event Custom|ClientHandleScopeInOut
  (params (InScope :type Boolean))
  ;[1 1 1] HANDLE SCOPE IN / OUT
  ;;[1 0.1179 0] INPUT FROM FIREARM SYSTEM
  (Variables|State|SetInScope InScope))

(event Custom|ClientHandleToggleFPMode
  (params (TogleOn :type Boolean))
  ;[1 1 1] TOGGLE FP MODE
  ;;[1 0.1179 0] INPUT FROM FIREARM SYSTEM
  (Variables|State|SetInFPMode TogleOn))

(event Custom|ServerCreateHitPointVFX
  (params (BlockingHit :type Boolean) (HitPointLocation :type Vector) (HitPointNormal :type Vector) (SurfaceType :type EPhysicalSurface%20Enum :default "SurfaceType_Default"))
  ;[1 1 1] HIT POINT VFX
  ;;[1 1 1] ServerCreateHitPointVFX
  (if BlockingHit
    (CallFunction|MulticastCreateHitPointVFX HitPointLocation HitPointNormal SurfaceType)))

(fn GetHitPointVFXs
  (return (.HitPointVFXs (Utilities|Struct|BreakS_WeaponLibraryVFXDesc (.VFX (Utilities|Struct|BreakS_WeaponLibraryDesc (Default|GetFirearmLibraryDesc (GETCOMPONENT|GetFirearmSystem))))))))

(fn GetHitPointVFXScale
  (return (.HitPointVFXScale (Utilities|Struct|BreakS_WeaponLibraryVFXDesc (.VFX (Utilities|Struct|BreakS_WeaponLibraryDesc (Default|GetFirearmLibraryDesc (GETCOMPONENT|GetFirearmSystem))))))))

(fn CreateHitPointVFX
  (params (HitPointLocation :type Vector) (HitPointNormal :type Vector) (SyrfaceType :type EPhysicalSurface%20Enum :default "SurfaceType_Default"))
  ;[1 1 1] hit sfx
  (for _array_element (GETFIREARMVALUES|GetHitPointVFXs)
    (if (Utilities|Enum|Equal(Enum) (.SurfacePhysType (Utilities|Struct|BreakS_WeaponHitPointVFXSFXDesc _array_element)) SyrfaceType)
      (LocalVariables|Setloc_hit_sfx (.SFX (Utilities|Struct|BreakS_WeaponHitPointVFXSFXDesc _array_element)))))
  (Effects|SpawnEmitteratLocation (LocalVariables|Getloc_hit_sfx) HitPointLocation (Math|Rotator|MakeRotfromX HitPointNormal) (GETFIREARMVALUES|GetHitPointVFXScale)))

(fn CreateHitPointDecal
  (params (HitPointLocation :type Vector) (HitPointNormal :type Vector) (SyrfaceType :type EPhysicalSurface%20Enum :default "SurfaceType_Default"))
  (bind _returnvalue (Math|Rotator|MakeRotfromX HitPointNormal))
  ;[1 1 1] hit decal
  (if (Utilities|Enum|Equal(Enum) "SurfaceType_Default" SyrfaceType)
    _
    (else
      _))
  (for _array_element (GETFIREARMVALUES|GetHitPointDecals)
    (if (Utilities|Enum|Equal(Enum) (.SurfaceType (Utilities|Struct|BreakS_WeaponDecalDesc _array_element)) SyrfaceType)
      (LocalVariables|Setloc_hit_decal (.Decal (Utilities|Struct|BreakS_WeaponDecalDesc _array_element)))))
  (bind _returnvalue_2 (Rendering|Decal|SpawnDecalatLocation (LocalVariables|Getloc_hit_decal) (GETFIREARMVALUES|GetHitPointDecalScale) HitPointLocation (Math|Rotator|MakeRotator (+ (.roll _returnvalue) 1.8e+02) (+ (.pitch _returnvalue) 1.8e+02) (.yaw _returnvalue)) 1e+01))
  (Utilities|IsValid _returnvalue_2
    (:Is%20Valid
      (Rendering|Components|Decal|SetFadeScreenSize _returnvalue_2 1e-05))))

(fn GetHitPointDecals
  (return (.HitPointDecals (Utilities|Struct|BreakS_WeaponLibraryVFXDesc (.VFX (Utilities|Struct|BreakS_WeaponLibraryDesc (Default|GetFirearmLibraryDesc (GETCOMPONENT|GetFirearmSystem))))))))

(fn GetHitPointDecalScale
  (return (.HitPointDecalScale (Utilities|Struct|BreakS_WeaponLibraryVFXDesc (.VFX (Utilities|Struct|BreakS_WeaponLibraryDesc (Default|GetFirearmLibraryDesc (GETCOMPONENT|GetFirearmSystem))))))))

(fn GetFirearmSystem
  (bind _self self)
  (bind _returnvalue (Components|GetOwner _self))
  (bind _returnvalue_2 (Actor|GetComponentbyClass _returnvalue "/Game/Blueprints/WeaponSystem/AC_WeaponSystem.AC_WeaponSystem_C"))
  (Utilities|IsValid _returnvalue_2
    (:Is%20Valid
      (return _returnvalue_2))))

(fn GetShotDelay
  (return (/ 1.0 (/ (Math|Conversions|ToFloat(Integer) (.FireRate (Utilities|Struct|BreakS_WeaponLibraryShootDesc (.Shoot (Utilities|Struct|BreakS_WeaponLibraryDesc (Default|GetFirearmLibraryDesc (GETCOMPONENT|GetFirearmSystem))))))) 6e+01))))

(fn GetTraceType
  (return (.TraceType (Utilities|Struct|BreakS_WeaponLibraryShootDesc (.Shoot (Utilities|Struct|BreakS_WeaponLibraryDesc (Default|GetFirearmLibraryDesc (GETCOMPONENT|GetFirearmSystem))))))))