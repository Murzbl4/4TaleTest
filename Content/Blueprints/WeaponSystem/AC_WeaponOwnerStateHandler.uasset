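; Weapon-owner component that tracks stance, ADS, movement, scope and first-person state and turns them into firearm handling modifiers.
; Server events from the weapon system combine the flags into a stance/aim/move state and multicast it.
; After a short replication delay, a looping timer linearly blends that state's firearm preset in ten steps over its transition time.
; It exposes recoil, spread, camera-shake and recoil-animation coefficients, notifying the weapon system each step.
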(event Custom|ServerHadleMovementOn
  ;[1 1 1] HANDLE OWNER STATE CHANGING
  ;;[1 0.1179 0] INPUT FROM FIREARMSYSTEM
  (Variables|OwnerState|SetInMove true)
  (CallFunction|ServerUpdateState)
  (CallFunction|ClientStartChangeInfState))

(event Custom|ServerHandleOwnerADSOn
  ;[1 1 1] HANDLE OWNER STATE CHANGING
  ;;[1 0.1179 0] INPUT FROM FIREARMSYSTEM
  (Variables|OwnerState|SetInADS true)
  (CallFunction|ServerUpdateState)
  (CallFunction|ClientStartChangeInfState))

(event Custom|ClientHandleScopeOnOff
  (params (InScope :type Boolean))
  ;[1 1 1] UPDATE SCOPE & FP MODE STATES
  ;;[1 0.1179 0] INPUT FROM FIREARMSYSTEM
  (Variables|OwnerState|SetInScope InScope))

(event Custom|ClientToggleFPModeOnOff
  (params (FPModeOn :type Boolean))
  ;[1 1 1] UPDATE SCOPE & FP MODE STATES
  ;;[1 0.1179 0] INPUT FROM FIREARMSYSTEM
  (Variables|OwnerState|SetInFPMode FPModeOn))

(event Custom|ServerHandleOwnerADSOff
  ;[1 1 1] HANDLE OWNER STATE CHANGING
  ;;[1 0.1179 0] INPUT FROM FIREARMSYSTEM
  (Variables|OwnerState|SetInADS false)
  (CallFunction|ServerUpdateState)
  (CallFunction|ClientStartChangeInfState))

(event Custom|ClientInterpChangeInfState
  (bind _oldinfdec (Variables|CurrentValues|GetOldInfDec))
  (bind _newinfdec (Variables|CurrentValues|GetNewInfDec))
  (bind (_recoil _spread _camerashake _recoilanimation) (Utilities|Struct|BreakS_WeaponOwnerStateInfluenceDesc _oldinfdec))
  (bind (_recoil_2 _spread_2 _camerashake_2 _recoilanimation_2) (Utilities|Struct|BreakS_WeaponOwnerStateInfluenceDesc _newinfdec))
  ;[1 1 1] INFLUENCE STATE CHANGING
  ;;[1 1 1] Interpolation Step
  ;;;[1 1 1] Stop condition. Preset was changed
  (if (Math|Float|NearlyEqual(Float) (Variables|CurrentValues|GetInterpTime) (.TransitionTime (Utilities|Struct|BreakS_WeaponOwnerStateInfluenceDesc (Variables|CurrentValues|GetNewInfDec))) 0.01)
    (Variables|CurrentValues|SetCurrentInfDec (Variables|CurrentValues|GetNewInfDec))
    (CallFunction|ClientStopChangeInfState)
    (CallFunction|ClientInfluenceIterated)
    (else
      ;;;[1 1 1] Interpolation Step
      (Variables|CurrentValues|SetInterpTime (+ (Variables|CurrentValues|GetInterpTime) (Variables|CurrentValues|GetInterpolationTimeStep)))
      (Variables|CurrentValues|SetCurrentInfDec (Utilities|Struct|MakeS_WeaponOwnerStateInfluenceDesc (Math|Interpolation|Ease "Linear" (/ (Variables|CurrentValues|GetInterpTime) (.TransitionTime (Utilities|Struct|BreakS_WeaponOwnerStateInfluenceDesc (Variables|CurrentValues|GetNewInfDec)))) _recoil _recoil_2) (Math|Interpolation|Ease "Linear" (/ (Variables|CurrentValues|GetInterpTime) (.TransitionTime (Utilities|Struct|BreakS_WeaponOwnerStateInfluenceDesc (Variables|CurrentValues|GetNewInfDec)))) _spread _spread_2) (Math|Interpolation|Ease "Linear" (/ (Variables|CurrentValues|GetInterpTime) (.TransitionTime (Utilities|Struct|BreakS_WeaponOwnerStateInfluenceDesc (Variables|CurrentValues|GetNewInfDec)))) _camerashake _camerashake_2) (Math|Interpolation|Ease "Linear" (/ (Variables|CurrentValues|GetInterpTime) (.TransitionTime (Utilities|Struct|BreakS_WeaponOwnerStateInfluenceDesc (Variables|CurrentValues|GetNewInfDec)))) _recoilanimation _recoilanimation_2) (.TransitionTime (Utilities|Struct|BreakS_WeaponOwnerStateInfluenceDesc (Variables|CurrentValues|GetNewInfDec)))))
      (CallFunction|ClientInfluenceIterated))))

(event Custom|ServerHandleOwnerCrouchOn
  ;[1 1 1] HANDLE OWNER STATE CHANGING
  ;;[1 0.1179 0] INPUT FROM FIREARMSYSTEM
  (Variables|OwnerState|SetInCrouch true)
  (CallFunction|ServerUpdateState)
  (CallFunction|ClientStartChangeInfState))

(event Custom|ServerHandleOwnerCrouchOff
  ;[1 1 1] HANDLE OWNER STATE CHANGING
  ;;[1 0.1179 0] INPUT FROM FIREARMSYSTEM
  (Variables|OwnerState|SetInCrouch false)
  (CallFunction|ServerUpdateState)
  (CallFunction|ClientStartChangeInfState))

(event Custom|ServerHandleOwnerProneOn
  ;[1 1 1] HANDLE OWNER STATE CHANGING
  ;;[1 0.1179 0] INPUT FROM FIREARMSYSTEM
  (Variables|OwnerState|SetInProne true)
  (CallFunction|ServerUpdateState)
  (CallFunction|ClientStartChangeInfState))

(event Custom|ServerHandleOwnerProneOff
  ;[1 1 1] HANDLE OWNER STATE CHANGING
  ;;[1 0.1179 0] INPUT FROM FIREARMSYSTEM
  (Variables|OwnerState|SetInProne false)
  (CallFunction|ServerUpdateState)
  (CallFunction|ClientStartChangeInfState))

(event Custom|ServerUpdateState
  ;[1 1 1] UPDATE OWNER COMMON STATE
  (if (Variables|OwnerState|GetInADS)
    (if (Variables|OwnerState|GetInProne)
      (if (not (Variables|OwnerState|GetInMove))
        (Variables|OwnerState|SetOwnerCommonState "NewEnumerator9")
        (CallFunction|MulticastUpdateState (Variables|OwnerState|GetOwnerCommonState) :!label _label))
      (elif (Variables|OwnerState|GetInCrouch)
        (if (Variables|OwnerState|GetInMove)
          (Variables|OwnerState|SetOwnerCommonState "NewEnumerator7")
          (goto _label)
          (else
            (Variables|OwnerState|SetOwnerCommonState "NewEnumerator6")
            (goto _label)))
        (elif (Variables|OwnerState|GetInMove)
          (Variables|OwnerState|SetOwnerCommonState "NewEnumerator3")
          (goto _label)
          (else
            (Variables|OwnerState|SetOwnerCommonState "NewEnumerator1")
            (goto _label)))))
    (elif (Variables|OwnerState|GetInProne)
      (if (not (Variables|OwnerState|GetInMove))
        (Variables|OwnerState|SetOwnerCommonState "NewEnumerator8")
        (goto _label))
      (elif (Variables|OwnerState|GetInCrouch)
        (if (Variables|OwnerState|GetInMove)
          (Variables|OwnerState|SetOwnerCommonState "NewEnumerator5")
          (goto _label)
          (else
            (Variables|OwnerState|SetOwnerCommonState "NewEnumerator4")
            (goto _label)))
        (elif (Variables|OwnerState|GetInMove)
          (Variables|OwnerState|SetOwnerCommonState "NewEnumerator2")
          (goto _label)
          (else
            (Variables|OwnerState|SetOwnerCommonState "NewEnumerator0")
            (goto _label)))))))

(event Custom|ClientStartChangeInfState
  (bind _firearmsystem (GETCOMPONENTS|GetFirearmSystem))
  (bind _firearmlibdesc (Default|GetFirearmLibraryDesc _firearmsystem))
  (bind _characterinfluence (Utilities|Struct|BreakS_WeaponLibraryDesc _firearmlibdesc))
  (bind (_standblind _standblindmove _standaim _standaimmove _crouchblind _crouchblindmove _crouchaim _crouchaimmove _proneblind _proneaim) (Utilities|Struct|BreakS_WeaponOwnerStateDesc _characterinfluence))
  ;[1 1 1] INFLUENCE STATE CHANGING
  ;;[1 1 1] Initialize Transition Values
  ;;;[1 1 1] Wait replicate OwnerCommonState value on all sides
  (Utilities|FlowControl|Delay 0.1)
  ;;;[1 1 1] Stop current interpolation if was, initialize old inf preset
  (CallFunction|ClientStopChangeInfState)
  (Variables|CurrentValues|SetOldInfDec (Variables|CurrentValues|GetCurrentInfDec))
  ;;;[1 1 1] Determine new inf preset
  (switch Utilities|FlowControl|Switch|SwitchonE_WeaponSystemOwnerCommonState (Variables|OwnerState|GetOwnerCommonState)
    (:NewEnumerator0
      (Variables|CurrentValues|SetNewInfDec _standblind))
    (:NewEnumerator2
      (Variables|CurrentValues|SetNewInfDec _standblindmove))
    (:NewEnumerator1
      (Variables|CurrentValues|SetNewInfDec _standaim))
    (:NewEnumerator3
      (Variables|CurrentValues|SetNewInfDec _standaimmove))
    (:NewEnumerator4
      (Variables|CurrentValues|SetNewInfDec _crouchblind))
    (:NewEnumerator5
      (Variables|CurrentValues|SetNewInfDec _crouchblindmove))
    (:NewEnumerator6
      (Variables|CurrentValues|SetNewInfDec _crouchaim))
    (:NewEnumerator7
      (Variables|CurrentValues|SetNewInfDec _crouchaimmove))
    (:NewEnumerator8
      (Variables|CurrentValues|SetNewInfDec _proneblind))
    (:NewEnumerator9
      (Variables|CurrentValues|SetNewInfDec _proneaim)))
  ;;;[1 1 1] Start Interp Step Event by time
  (Variables|CurrentValues|SetInterpolationTimeStep (/ (.TransitionTime (Utilities|Struct|BreakS_WeaponOwnerStateInfluenceDesc (Variables|CurrentValues|GetNewInfDec))) 1e+01))
  (if (> (Variables|CurrentValues|GetInterpolationTimeStep) 0.0)
    (Utilities|Time|SetTimerbyFunctionName 0 "ClientInterpChangeInfState" (Variables|CurrentValues|GetInterpolationTimeStep) true)))

(event Custom|ClientStopChangeInfState
  ;[1 1 1] INFLUENCE STATE CHANGING
  ;;[1 1 1] Stop Interpolated Transition
  (Variables|CurrentValues|SetInterpTime 0.0)
  (Utilities|Time|ClearTimerbyFunctionName 0 "ClientInterpChangeInfState"))

(event Custom|ServerHadleMovementOff
  ;[1 1 1] HANDLE OWNER STATE CHANGING
  ;;[1 0.1179 0] INPUT FROM FIREARMSYSTEM
  (Variables|OwnerState|SetInMove false)
  (CallFunction|ServerUpdateState)
  (CallFunction|ClientStartChangeInfState))

(event Custom|ClientHandleInitFirearm
  (bind _firearmsystem (GETCOMPONENTS|GetFirearmSystem))
  (bind _firearmlibdesc (Default|GetFirearmLibraryDesc _firearmsystem))
  (bind _characterinfluence (Utilities|Struct|BreakS_WeaponLibraryDesc _firearmlibdesc))
  (bind (_standblind _standblindmove _standaim _standaimmove _crouchblind _crouchblindmove _crouchaim _crouchaimmove _proneblind _proneaim) (Utilities|Struct|BreakS_WeaponOwnerStateDesc _characterinfluence))
  ;[1 1 1] IN INIT FIREARM
  ;;[1 0.1179 0] INPUT FROM FIREARMSYSTEM
  ;;[1 1 1] Determine new inf preset
  (switch Utilities|FlowControl|Switch|SwitchonE_WeaponSystemOwnerCommonState (Variables|OwnerState|GetOwnerCommonState)
    (:NewEnumerator0
      (Variables|CurrentValues|SetCurrentInfDec _standblind))
    (:NewEnumerator2
      (Variables|CurrentValues|SetCurrentInfDec _standblindmove))
    (:NewEnumerator1
      (Variables|CurrentValues|SetCurrentInfDec _standaim))
    (:NewEnumerator3
      (Variables|CurrentValues|SetCurrentInfDec _standaimmove))
    (:NewEnumerator4
      (Variables|CurrentValues|SetCurrentInfDec _crouchblind))
    (:NewEnumerator5
      (Variables|CurrentValues|SetCurrentInfDec _crouchblindmove))
    (:NewEnumerator6
      (Variables|CurrentValues|SetCurrentInfDec _crouchaim))
    (:NewEnumerator7
      (Variables|CurrentValues|SetCurrentInfDec _crouchaimmove))
    (:NewEnumerator8
      (Variables|CurrentValues|SetCurrentInfDec _proneblind))
    (:NewEnumerator9
      (Variables|CurrentValues|SetCurrentInfDec _proneaim))))

(event Custom|MulticastUpdateState
  (params (OwnerCommonState :type E_WeaponSystemOwnerCommonState%20Enum :default "NewEnumerator0"))
  ;[1 1 1] UPDATE OWNER COMMON STATE
  ;;[1 1 1] MulticastUpdateState
  (Variables|OwnerState|SetOwnerCommonState OwnerCommonState))

(event Custom|ClientInfluenceIterated
  ;[1 1 1] INFLUENCE INTERETED EVENT
  ;;[0.9739 1 0] BI OUTPUT TO FirearmSystem
  (Default|ClientUpdateOwnerInfluencesIterated (GETCOMPONENTS|GetFirearmSystem)))

(event EventBeginPlay
  ;[1 1 1] EVENT BEGIN PLAY
  (Variables|OwnerState|SetOwnerCommonState "NewEnumerator0"))

(fn GetCurrentRecoilCoeff
  (return (.Recoil (Utilities|Struct|BreakS_WeaponOwnerStateInfluenceDesc (Variables|CurrentValues|GetCurrentInfDec)))))

(fn GetCurrentSpreadCoeff
  (return (.Spread (Utilities|Struct|BreakS_WeaponOwnerStateInfluenceDesc (Variables|CurrentValues|GetCurrentInfDec)))))

(fn GetCurrentCameraShakeCoeff
  (return (.CameraShake (Utilities|Struct|BreakS_WeaponOwnerStateInfluenceDesc (Variables|CurrentValues|GetCurrentInfDec)))))

(fn GetCurrentRecoilAnimationCoeff
  (return (.RecoilAnimation (Utilities|Struct|BreakS_WeaponOwnerStateInfluenceDesc (Variables|CurrentValues|GetCurrentInfDec)))))

(fn GetFirearmSystem
  (bind _self self)
  (bind _returnvalue (Components|GetOwner _self))
  (bind _returnvalue_2 (Actor|GetComponentbyClass _returnvalue "/Game/Blueprints/WeaponSystem/AC_WeaponSystem.AC_WeaponSystem_C"))
  (Utilities|IsValid _returnvalue_2
    (:Is%20Valid
      (return _returnvalue_2))))

(fn GetinProne
  (return (Variables|OwnerState|GetInProne)))

(fn GetinADS
  (return (Variables|OwnerState|GetInADS)))

(fn GetinCrouch
  (return (Variables|OwnerState|GetInCrouch)))

(fn GetinMove
  (return (Variables|OwnerState|GetInMove)))

(fn GetOwnerCommonState
  (return (Variables|OwnerState|GetOwnerCommonState)))

(fn GetinScope
  (return (Variables|OwnerState|GetInScope)))

(fn GetinFPMode
  (return (Variables|OwnerState|GetInFPMode)))