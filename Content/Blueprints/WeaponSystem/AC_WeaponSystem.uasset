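; Hub component of the weapon system on a BP_BasePawn, routing firearm events between the character, the weapon actor and specialised sub-components.
; On authority it spawns shooting, spread, owner-state, hitscan, VFX, sound and damage components, and it initialises equipped firearms against DT_WeaponLibrary.
; Input drives shooting and reload, spread feeds hitscan traces, and hits fan out to character, sound and damage.
; Client events report to the character, while server events update ammo.
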(event Custom|ServerHandleOwnerSprintOn
  ;[1 1 1] INPUT OWNER STATE
  ;;[1 0.1179 0] INPUT FROM CHARACTER
)

(event Custom|ServerHandleOwnerSprintOff
  ;[1 1 1] INPUT OWNER STATE
  ;;[1 0.1179 0] INPUT FROM CHARACTER
)

(event Custom|ClientMainReloadFinish
  ;[1 1 1] INPUTS FROM SHOOTING CONTROLLER
  ;;[1 1 1] Main Reload
  ;;;[1 0.1179 0] INPUT FROM SHOOTING CONTROLLER
  (CallFunction|ClientFirearmEvent "NewEnumerator3")
  (CallFunction|ServerMainReloadFinish)
  ;;;[1 0.6824 0] TO CHARACTER COMMON
  (Default|ClientMainReloadOff (GETCOMPONENTS|GetCharacterCommon)))

(event Custom|ClientHandleAnimEventReloadAction
  (params (Index :type Integer))
  ;[1 1 1] INPUT ON HANDLE RELOAD ANIM EVENT
  ;;[1 0.1179 0] INPUT FROM ABP CHARACTER BASE
  (Default|ClientHandleAnimEventReloadAction (GETCOMPONENTS|GetFirearmSoundController) Index))

(event Custom|ClientHandleShellOnExtraReload
  ;[1 1 1] INPUT ON HANDLE RELOAD ANIM EVENT
  ;;[1 0.1179 0] INPUT FROM ABP CHARACTER BASE
  (Default|ClientHandleAnimEventReloadAction (GETCOMPONENTS|GetFirearmSoundController)))

(event Custom|ClientMainReloadCyclicStartToPos
  ;[1 1 1] INPUTS FROM SHOOTING CONTROLLER
  ;;[1 1 1] Cyclic Main Reload
  ;;;[1 0.1179 0] INPUT FROM SHOOTING CONTROLLER
  (CallFunction|ClientFirearmEvent "NewEnumerator5"))

(event Custom|ClientMainReloadCyclicStart
  ;[1 1 1] INPUTS FROM SHOOTING CONTROLLER
  ;;[1 1 1] Cyclic Main Reload
  ;;;[1 0.1179 0] INPUT FROM SHOOTING CONTROLLER
  (CallFunction|ClientFirearmEvent "NewEnumerator6"))

(event Custom|ClientMainReloadCyclicStop
  ;[1 1 1] INPUTS FROM SHOOTING CONTROLLER
  ;;[1 1 1] Cyclic Main Reload
  ;;;[1 0.1179 0] INPUT FROM SHOOTING CONTROLLER
  (CallFunction|ClientFirearmEvent "NewEnumerator7"))

(event Custom|ClientMainReloadCyclicEndToPos
  ;[1 1 1] INPUTS FROM SHOOTING CONTROLLER
  ;;[1 1 1] Cyclic Main Reload
  ;;;[1 0.1179 0] INPUT FROM SHOOTING CONTROLLER
  (CallFunction|ClientFirearmEvent "NewEnumerator8"))

(event Custom|ServerShotHappened
  ;[1 1 1] INPUTS FROM SHOOTING CONTROLLER
  ;;[1 1 1] Main
  ;;;[1 0.6824 0] TO FIREARM ACTOR
  (Default|ServerUpdateAmmoinCliponShot (Variables|COMMON|GetFirearmItemCommon)))

(event Custom|ServerInitializeFirearmItem
  (params (FirearmActor :type Actor%20Object%20Reference))
  ;[1 1 1] INITIALIZE FIREARM
  ;;[1 0.1179 0] INPUT FROM CHARACTER
  ;;[1 1 1] Initialize & Check Valid Actor
  (bind _asbp_firearm_actor_common (Utilities|Casting|CastToBP_WeaponActorCommon FirearmActor)
    (:then
      (bind _output_get (Variables|COMMON|SetFirearmItemCommon _asbp_firearm_actor_common))
      (Variables|COMMON|SetFirearmTag (Variables|/Game/Blueprints/WeaponSystem/BP_WeaponActorCommon.BP_WeaponActorCommon_C|GetFirearmTag _output_get))
      (bind _returnvalue (Class|DataTableFunctionLibrary|DoesDataTableRowExist "/Game/Blueprints/WeaponBase/DT_WeaponLibrary.DT_WeaponLibrary" (Variables|COMMON|GetFirearmTag)))
      (if _returnvalue
        (Utilities|FlowControl|Delay 0.1)
        ;;[1 1 1] Initialize Firearm System Components
        (Default|ClientHandleInitFirearm (GETCOMPONENTS|GetFirearmOwnerStateHandler))
        (Default|ClientHandleUpdateMinSpreadonInitFirearm (GETCOMPONENTS|GetFirearmSpreadController))
        ;;[1 1 1] Check condition for main reload / extra reload on init firearm
        (if (== (Default|GetCurrentAmmoinClip (Variables|COMMON|GetFirearmItemCommon)) 0)
          (Default|ClientRequestedMainReload (GETCOMPONENTS|GetFirearmShootingController)))
        (else
          (Utilities|DebugMessage "Firearm Item Tag is not found in Firearm Library"))))
    (:CastFailed
      (Utilities|DebugMessage "Actor on init is not child of FirearmItemCommon"))))

(event Custom|ServerChildHandleSwitchFirearmFinish
  ;[1 1 1] SWITCH FIREARMS
  ;;[0.1778 0 1] PARENT OUTPUT EVENT
)

(event Custom|ClientHandleReadyToSingleShot
  (params (TraceStartPoint :type Vector) (TraceEndPoint :type Vector))
  ;[1 1 1] INPUTS FROM SPREAD CONTROLLLER
  ;;[1 0.1179 0] INPUT FROM FIREARM SPREAD CONTROLLER
  ;;[1 0.6824 0] TO FIREARM HITSCAN
  (Default|ClientHandleCreateSingleLineTrace (GETCOMPONENTS|GetFirearmHitScan) TraceStartPoint TraceEndPoint))

(event Custom|ClientHandleReadyToMultiShot
  (params (MultiTraces :type Array%20of%20S%20Weapon%20Multi%20Trace%20Desc%20Structures))
  ;[1 1 1] INPUTS FROM SPREAD CONTROLLLER
  ;;[1 0.1179 0] INPUT FROM FIREAM SPREAD CONTROLLER
  ;;[1 0.6824 0] TO FIREARM HITSCAN
  (Default|ClientHandleCreateMultiLineTrace (GETCOMPONENTS|GetFirearmHitScan) MultiTraces))

(event Custom|ServerMainReloadFinish
  ;[1 1 1] INPUTS FROM SHOOTING CONTROLLER
  ;;[1 1 1] Main Reload
  ;;;[1 0.6824 0] TO FIREARM ACTOR
  (Default|ServerUpdateAmmoonMainReload (Variables|COMMON|GetFirearmItemCommon)))

(event Custom|ClientInputPressedShooting
  ;[1 1 1] INPUTS FROM CHARACTER
  ;;[1 0.1179 0] INPUT FROM CHARACTER
  ;;[1 0.6824 0] TO FIREARM SHOOTING CONTROLLER
  (Default|ClientShootPressed (GETCOMPONENTS|GetFirearmShootingController)))

(event Custom|ClientUpdateOwnerInfluencesIterated
  ;[1 1 1] INPUT FROM OWNER STATE HANDLER
  ;;[1 0.1179 0] INPUT FROM OWNER STATE HANDLER
  (Default|ClientHandleUpdateSpreadInfonIteratationStep (GETCOMPONENTS|GetFirearmSpreadController)))

(event Custom|ClientInputReloadTrigger
  ;[1 1 1] INPUTS FROM CHARACTER
  ;;[1 0.1179 0] INPUT FROM CHARACTER
  (Default|ClientRequestedMainReload (GETCOMPONENTS|GetFirearmShootingController)))

(event Custom|ClientFirearmEvent
  (params (FirearmEventType :type E_GL_WeaponEventType%20Enum :default "NewEnumerator0"))
  ;[1 1 1] OUTPUTS TO CHARACTER
  ;;[1 0.6824 0] TO CHARACTER COMMON
  (Default|ClientHandleFirearmEvent (GETCOMPONENTS|GetCharacterCommon) FirearmEventType))

(event Custom|ServerHandleOwnerADSOn
  ;[1 1 1] INPUT OWNER STATE
  ;;[1 0.1179 0] INPUT FROM CHARACTER
  (Default|ServerHandleOwnerADSon (GETCOMPONENTS|GetFirearmOwnerStateHandler))
  (Default|ClientPlayZoominSound (GETCOMPONENTS|GetFirearmSoundController)))

(event Custom|ClientMultiTraceCreated
  (params (MultiTraceDesc :type Array%20of%20S%20Weapon%20Hit%20Scan%20Desc%20Structures))
  ;[1 1 1] INPUT FROM HIT SCAN
  ;;[1 0.1179 0] INPUT FROM FIREARM HIT SCAN
  ;;[1 0.6824 0] TO CHARACTER COMMON
  (Default|ClientHandleMultiTraceCreated (GETCOMPONENTS|GetCharacterCommon) MultiTraceDesc)
  ;;[1 0.6824 0] TO FIREARM SOUND CONTROLLER
  (Default|ClientHandlePlayerSoundonMultiHit (GETCOMPONENTS|GetFirearmSoundController) MultiTraceDesc)
  ;;[1 0.6824 0] TO FIREARM DAMAGE HANDLER
  (Default|ServerHandleMultiHit (GETCOMPONENTS|GetFirearmDamageHandler) MultiTraceDesc))

(event Custom|ServerHandleOwnerCrouchOff
  ;[1 1 1] INPUT OWNER STATE
  ;;[1 0.1179 0] INPUT FROM CHARACTER
  (Default|ServerHandleOwnerCrouchOff (GETCOMPONENTS|GetFirearmOwnerStateHandler)))

(event Custom|ClientSingleTraceCreated
  (params (SingleTraceDesc :type S%20Weapon%20Hit%20Scan%20Desc%20Structure))
  ;[1 1 1] INPUT FROM HIT SCAN
  ;;[1 0.1179 0] INPUT FROM FIREARM HIT SCAN
  ;;[1 0.6824 0] TO CHARACTER COMMON
  (Default|ClientHandleSingleTraceCreated (GETCOMPONENTS|GetCharacterCommon) SingleTraceDesc)
  ;;[1 0.6824 0] TO FIREARM SOUND CONTROLLER
  (Default|ClientHandlePlayerSoundonSingleHit (GETCOMPONENTS|GetFirearmSoundController) SingleTraceDesc)
  ;;[1 0.6824 0] TO FIREARM DAMAGE HANDLER
  (Default|ServerHandleSingleHit (GETCOMPONENTS|GetFirearmDamageHandler) SingleTraceDesc))

(event Custom|ServerHandleSwitchFirearmFinish
  ;[1 1 1] SWITCH FIREARMS
)

(event Custom|ClientInputReleasedShooting
  ;[1 1 1] INPUTS FROM CHARACTER
  ;;[1 0.1179 0] INPUT FROM CHARACTER
  (Default|ClientShootReleased (GETCOMPONENTS|GetFirearmShootingController))
  (CallFunction|ClientFirearmEvent "NewEnumerator12"))

(event Custom|ServerHandleOwnerProneOff
  ;[1 1 1] INPUT OWNER STATE
  ;;[1 0.1179 0] INPUT FROM CHARACTER
  (Default|ServerHandleOwnerProneOff (GETCOMPONENTS|GetFirearmOwnerStateHandler)))

(event Custom|ServerHandleOwnerCrouchOn
  ;[1 1 1] INPUT OWNER STATE
  ;;[1 0.1179 0] INPUT FROM CHARACTER
  (Default|ServerHandleOwnerCrouchon (GETCOMPONENTS|GetFirearmOwnerStateHandler)))

(event Custom|ServerHandleOwnerMoveOff
  ;[1 1 1] INPUT OWNER STATE
  ;;[1 0.1179 0] INPUT FROM CHARACTER
  (Default|ServerHadleMovementOff (GETCOMPONENTS|GetFirearmOwnerStateHandler)))

(event Custom|ServerHandleOwnerMoveOn
  ;[1 1 1] INPUT OWNER STATE
  ;;[1 0.1179 0] INPUT FROM CHARACTER
  (Default|ServerHadleMovementon (GETCOMPONENTS|GetFirearmOwnerStateHandler)))

(event Custom|ClientMainReloadCanceled
  ;[1 1 1] INPUTS FROM SHOOTING CONTROLLER
  ;;[1 1 1] Main Reload
  ;;;[1 0.1179 0] INPUT FROM SHOOTING CONTROLLER
  (CallFunction|ClientFirearmEvent "NewEnumerator4"))

(event Custom|ClientShotHappened
  ;[1 1 1] INPUTS FROM SHOOTING CONTROLLER
  ;;[1 1 1] Main
  ;;;[1 0.1179 0] INPUT FROM SHOOTING CONTROLLER
  (CallFunction|ClientFirearmEvent "NewEnumerator0")
  (CallFunction|ServerShotHappened)
  (Default|ClientHandleUpdateSpreadonShot (GETCOMPONENTS|GetFirearmSpreadController))
  (Default|ClientHandlePlayerSoundonShot (GETCOMPONENTS|GetFirearmSoundController)))

(event Custom|HandleSwitchFirearmsDown
  (params (HalfSwitchTime :type Float%20%28double-precision%29))
  ;[1 1 1] SWITCH FIREARMS
  ;;[1 0.1179 0] BI INPUT FROM CHARACTER
  (Default|ClientPlaySwitchDownSound (GETCOMPONENTS|GetFirearmSoundController)))

(event Custom|HandleSwitchFirearmsUp
  (params (HalfSwitchTime :type Float%20%28double-precision%29))
  ;[1 1 1] SWITCH FIREARMS
  ;;[1 0.1179 0] BI INPUT FROM CHARACTER
  (Default|ClientPlaySwitchUpSound (GETCOMPONENTS|GetFirearmSoundController)))

(event Custom|HandleSwitchFirearmsFinish
  ;[1 1 1] SWITCH FIREARMS
  ;;[1 0.1179 0] BI INPUT FROM CHARACTER
  (CallFunction|ServerHandleSwitchFirearmFinish)
  (CallFunction|ServerChildHandleSwitchFirearmFinish))

(event Custom|ClientShotDelayEnded
  ;[1 1 1] INPUTS FROM SHOOTING CONTROLLER
  ;;[1 1 1] Main
  ;;;[1 0.1179 0] INPUT FROM SHOOTING CONTROLLER
  (CallFunction|ClientFirearmEvent "NewEnumerator1"))

(event Custom|ServerHandleOwnerADSOff
  ;[1 1 1] INPUT OWNER STATE
  ;;[1 0.1179 0] INPUT FROM CHARACTER
  (Default|ServerHandleOwnerADSOff (GETCOMPONENTS|GetFirearmOwnerStateHandler))
  (Default|ClientPlayZoomOutSound (GETCOMPONENTS|GetFirearmSoundController)))

(event Custom|ServerHandleOwnerProneOn
  ;[1 1 1] INPUT OWNER STATE
  ;;[1 0.1179 0] INPUT FROM CHARACTER
  (Default|ServerHandleOwnerProneon (GETCOMPONENTS|GetFirearmOwnerStateHandler)))

(event Custom|ClientFirearmsAmmoEmpty
  ;[1 1 1] INPUTS FROM SHOOTING CONTROLLER
  ;;[1 1 1] Main
  ;;;[1 0.1179 0] INPUT FROM SHOOTING CONTROLLER
  (CallFunction|ClientFirearmEvent "NewEnumerator11"))

(event Custom|ClientMainReloadStart
  ;[1 1 1] INPUTS FROM SHOOTING CONTROLLER
  ;;[1 1 1] Main Reload
  ;;;[1 0.1179 0] INPUT FROM SHOOTING CONTROLLER
  (CallFunction|ClientFirearmEvent "NewEnumerator2")
  ;;;[1 0.6824 0] TO CHARACTER COMMON
  (Default|ClientMainReloadon (GETCOMPONENTS|GetCharacterCommon)))

(event EventBeginPlay
  ;[1 1 1] EVENT BEGIN PLAY
  (Networking|SwitchHasAuthority
    (:Authority
      ;;[1 1 1] Create FirearmShootingController
      (Game|AddComponentbyClass (Components|GetOwner self) "/Game/Blueprints/WeaponSystem/AC_WeaponShootingController.AC_WeaponShootingController_C")
      ;;[1 1 1] Create FirearmSpreadController
      (Game|AddComponentbyClass (Components|GetOwner self) "/Game/Blueprints/WeaponSystem/AC_WeaponSpreadController.AC_WeaponSpreadController_C")
      ;;[1 1 1] Create FirearmOwnerStateHandler
      (Game|AddComponentbyClass (Components|GetOwner self) "/Game/Blueprints/WeaponSystem/AC_WeaponOwnerStateHandler.AC_WeaponOwnerStateHandler_C")
      ;;[1 1 1] Create FirearmHitScan
      (Game|AddComponentbyClass (Components|GetOwner self) "/Game/Blueprints/WeaponSystem/AC_WeaponHitScan.AC_WeaponHitScan_C")
      ;;[1 1 1] Create FirearmVFXController
      (Game|AddComponentbyClass (Components|GetOwner self) "/Game/Blueprints/WeaponSystem/AC_WeaponVFXController.AC_WeaponVFXController_C")
      ;;[1 1 1] Create FirearmSoundController
      (Game|AddComponentbyClass (Components|GetOwner self) "/Game/Blueprints/WeaponSystem/AC_WeaponSoundController.AC_WeaponSoundController_C")
      ;;[1 1 1] Create FirearmDamageHandler
      (Game|AddComponentbyClass (Components|GetOwner self) "/Game/Blueprints/WeaponSystem/AC_WeaponDamage.AC_WeaponDamage_C"))))

(fn GetFirearmLibraryDesc
  (bind _returnvalue (Utilities|GetDataTableRow "/Game/Blueprints/WeaponBase/DT_WeaponLibrary.DT_WeaponLibrary" (Variables|COMMON|GetFirearmTag))
    (:then
      (return _returnvalue))))

(fn GetFirearmOwnerStateHandler
  (bind _self self)
  (bind _returnvalue (Components|GetOwner _self))
  (bind _returnvalue_2 (Actor|GetComponentbyClass _returnvalue "/Game/Blueprints/WeaponSystem/AC_WeaponOwnerStateHandler.AC_WeaponOwnerStateHandler_C"))
  (Utilities|IsValid _returnvalue_2
    (:Is%20Valid
      (return _returnvalue_2))))

(fn GetFirearmSpreadController
  (bind _self self)
  (bind _returnvalue (Components|GetOwner _self))
  (bind _returnvalue_2 (Actor|GetComponentbyClass _returnvalue "/Game/Blueprints/WeaponSystem/AC_WeaponSpreadController.AC_WeaponSpreadController_C"))
  (Utilities|IsValid _returnvalue_2
    (:Is%20Valid
      (return _returnvalue_2))))

(fn GetFirearmShootingController
  (bind _self self)
  (bind _returnvalue (Components|GetOwner _self))
  (bind _returnvalue_2 (Actor|GetComponentbyClass _returnvalue "/Game/Blueprints/WeaponSystem/AC_WeaponShootingController.AC_WeaponShootingController_C"))
  (Utilities|IsValid _returnvalue_2
    (:Is%20Valid
      (return _returnvalue_2))))

(fn GetFirearmItemCommon
  (return (Variables|COMMON|GetFirearmItemCommon)))

(fn GetFirearmSoundController
  (bind _self self)
  (bind _returnvalue (Components|GetOwner _self))
  (bind _returnvalue_2 (Actor|GetComponentbyClass _returnvalue "/Game/Blueprints/WeaponSystem/AC_WeaponSoundController.AC_WeaponSoundController_C"))
  (Utilities|IsValid _returnvalue_2
    (:Is%20Valid
      (return _returnvalue_2))))

(fn GetFirearmHitScan
  (bind _self self)
  (bind _returnvalue (Components|GetOwner _self))
  (bind _returnvalue_2 (Actor|GetComponentbyClass _returnvalue "/Game/Blueprints/WeaponSystem/AC_WeaponHitScan.AC_WeaponHitScan_C"))
  (Utilities|IsValid _returnvalue_2
    (:Is%20Valid
      (return _returnvalue_2))))

(fn GetFirearmDamageHandler
  (bind _self self)
  (bind _returnvalue (Components|GetOwner _self))
  (bind _returnvalue_2 (Actor|GetComponentbyClass _returnvalue "/Game/Blueprints/WeaponSystem/AC_WeaponDamage.AC_WeaponDamage_C"))
  (Utilities|IsValid _returnvalue_2
    (:Is%20Valid
      (return _returnvalue_2))))

(fn GetCharacterCommon
  (Utilities|IsValid (Components|GetOwner self)
    (:Is%20Valid
      (bind _asbp_base_pawn (Utilities|Casting|CastToBP_BasePawn (Components|GetOwner self)))
      (return _asbp_base_pawn))))

(fn GetFirearmVFXController
  (bind _self self)
  (bind _returnvalue (Components|GetOwner _self))
  (bind _returnvalue_2 (Actor|GetComponentbyClass _returnvalue "/Game/Blueprints/WeaponSystem/AC_WeaponVFXController.AC_WeaponVFXController_C"))
  (Utilities|IsValid _returnvalue_2
    (:Is%20Valid
      (return _returnvalue_2))))