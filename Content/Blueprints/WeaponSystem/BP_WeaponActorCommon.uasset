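; Common firearm actor that tracks clip ammo, plays weapon mesh animations and exposes item data to the inventory system.
; Stats come from DT_WeaponLibrary by FirearmTag through getter functions.
; Server events decrement ammo on shots and refill from inventory reserves on reload, writing the remainder back.
; Unless simple animation is set, server events multicast third-person shot and reload animations, rate-scaled to weapon timings, and clip bone hiding.
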(event Custom|ServerUpdateAmmoInClipOnShot
  ;[1 1 1] UPDATE AMMO
  ;;[1 0.1179 0] INPUT FROM Weapon SYSTEM
  (Variables|COMMON|SetCurrentAmmoInClip (- (Variables|COMMON|GetCurrentAmmoInClip) 1)))

(event Custom|ServerTPHandleShotHappened
  ;[1 1 1] Weapon EVENTS
  ;;[1 1 1] ServerTPHandleShotHappened
  (if (not (GETFIREARMVALUES|GetUseSimpleAnimMethod))
    (CallFunction|MulticastTPHandleShotHappened)))

(event Custom|MulticastTPMainReloadStart
  (bind _firearmownerstatehandler (GETCOMPONENTS|GeFirearmOwnerStateHandler))
  (bind _firearm_main_reload_stand (Variables|PUBLICSETTINGS|GetFirearm%20Main%20Reload%20Stand))
  (bind _firearm_main_reload_prone (Variables|PUBLICSETTINGS|GetFirearm%20Main%20Reload%20Prone))
  (bind _inprone (Default|GetinProne _firearmownerstatehandler))
  (bind _returnvalue (select _inprone _firearm_main_reload_prone _firearm_main_reload_stand))
  ;[1 1 1] Weapon EVENTS
  ;;[1 1 1] MulticastTPMainReloadStart
  (Utilities|IsValid _returnvalue
    (:Is%20Valid
      (Components|Animation|PlayAnimation (Variables|Default|GetFirearmMesh) _returnvalue false)
      (Components|Timeline|SetPlayRate (Variables|Default|GetFirearmMesh) (/ (Animation|GetPlayLength _returnvalue) (GETFIREARMVALUES|GetMainReloadTime)))
      (Utilities|FlowControl|Delay (GETFIREARMVALUES|GetMainReloadTime))
      (Audio|Components|Audio|Stop (Variables|Default|GetFirearmMesh)))))

(event Custom|ServerHandleClipInHandTP
  ;[1 1 1] CLIP OBJ EVENTS FOR TP
  ;;[1 1 1] ServerHandleClipInHandTP
  ;;;[1 0.1179 0] INPUT FROM CHARACTER TP / FP
  (if (not (GETFIREARMVALUES|GetUseSimpleAnimMethod))
    (Utilities|IsValid (Components|GetOwner)
      (:Is%20Valid
        (CallFunction|MulticastHandleClipinHandTP)))))

(event Custom|ServerHandleTPFirearmEvent
  (params (FirearmEventType :type E_GL_WeaponEventType%20Enum :default "NewEnumerator0"))
  ;[1 1 1] Weapon EVENTS
  ;;[1 1 1] ServerHandleTPFirearmEvent
  ;;;[1 0.1179 0] INPUT FROM CHARACTER TP / FP
  (switch Utilities|FlowControl|Switch|SwitchonE_GL_WeaponEventType FirearmEventType
    (:NewEnumerator0
      (CallFunction|ServerTPHandleShotHappened))
    (:NewEnumerator2
      (CallFunction|ServerTPMainReloadStart))))

(event Custom|MulticastHandleClipInHandTP
  ;[1 1 1] CLIP OBJ EVENTS FOR TP
  ;;[1 1 1] MulticastHandleClipInHandTP
  ;;;[1 1 1] UnHide Clip
  (Components|SkinnedMesh|UnHideBonebyName (Variables|Default|GetFirearmMesh) (GETFIREARMVALUES|GetReloadAttachBone)))

(event Custom|MulticastTPHandleShotHappened
  ;[1 1 1] Weapon EVENTS
  ;;[1 1 1] MulticastTPHandleShotHappened
  (Utilities|IsValid (Variables|PUBLICSETTINGS|GetFirearm%20Shot)
    (:Is%20Valid
      (Components|Animation|PlayAnimation (Variables|Default|GetFirearmMesh) (Variables|PUBLICSETTINGS|GetFirearm%20Shot) false)
      (Components|Timeline|SetPlayRate (Variables|Default|GetFirearmMesh) (/ (Animation|GetPlayLength (Variables|PUBLICSETTINGS|GetFirearm%20Shot)) (Math|Float|Clamp(Float) (GETFIREARMVALUES|GetShotDelay) 0.05 0.1)))
      (Utilities|FlowControl|Delay (GETFIREARMVALUES|GetShotDelay))
      (Components|Animation|PlayAnimation (Variables|Default|GetFirearmMesh) (Variables|PUBLICSETTINGS|GetFirearm%20Idle%20State%20) false)
      (Audio|Components|Audio|Stop (Variables|Default|GetFirearmMesh)))))

(event Custom|ClientHandleUpdateVisibilityMeshItem
  (params (NewVisibilityMode :type E_InventoryItemVisibilityMode%20Enum :default "NewEnumerator0"))
  ;[1 1 1] HANDLE UPDATE VISIBILITY MESH ITEM FOR OWNER
  (switch Utilities|FlowControl|Switch|SwitchonE_InventoryItemVisibilityMode NewVisibilityMode
    (:NewEnumerator0
      ;;[1 1 1] Show Mesh & Show Cast Hidden Shadows
      (Rendering|SetVisibility (Variables|Default|GetFirearmMesh) true false)
      (Class|PrimitiveComponent|SetCastHiddenShadow (Variables|Default|GetFirearmMesh) true))
    (:NewEnumerator2
      ;;[1 1 1] Show Mesh & Hide Cast Hidden Shadows
      (Rendering|SetVisibility (Variables|Default|GetFirearmMesh) true false)
      (Class|PrimitiveComponent|SetCastHiddenShadow (Variables|Default|GetFirearmMesh) false))
    (:NewEnumerator1
      ;;[1 1 1] Hide Mesh & Show Cast Hidden Shadows
      (Rendering|SetVisibility (Variables|Default|GetFirearmMesh) false false)
      (Class|PrimitiveComponent|SetCastHiddenShadow (Variables|Default|GetFirearmMesh) true))))

(event Custom|ServerUpdateAmmoOnMainReload
  ;[1 1 1] UPDATE AMMO
  ;;[1 0.1179 0] INPUT FROM Weapon SYSTEM
  (bind (_updatedresammotype _updatedresammocount) (COMMON|UpdateAmmoonMainReload))
  ;;[1 0.6824 0] TO INVENTORY SYSTEM
  (Default|ServerUpdateAmmoRes (GETCOMPONENTS|GeInventorySystem) _updatedresammotype _updatedresammocount))

(event Custom|ServerTPMainReloadStart
  ;[1 1 1] Weapon EVENTS
  ;;[1 1 1] ServerTPMainReloadStart
  (if (not (GETFIREARMVALUES|GetUseSimpleAnimMethod))
    (CallFunction|MulticastTPMainReloadStart)))

(event Custom|ServerHandleClipEndFollowTP
  ;[1 1 1] CLIP OBJ EVENTS FOR TP
  ;;[1 1 1] ServerHandleClipEndFollowTP
  ;;;[1 0.1179 0] INPUT FROM CHARACTER TP / FP
  (if (not (GETFIREARMVALUES|GetUseSimpleAnimMethod))
    (Utilities|IsValid (Components|GetOwner)
      (:Is%20Valid
        (CallFunction|MulticastHandleClipEndFollowTP true)))))

(event Custom|MulticastHandleClipEndFollowTP
  (params (With%20Hide%20Clip%20for%20Owner :type Boolean))
  ;[1 1 1] CLIP OBJ EVENTS FOR TP
  ;;[1 1 1] MulticastHandleClipEndFollowTP
  (Variables|COMMON|SetWith%20Hide%20Clip%20for%20Owner With%20Hide%20Clip%20for%20Owner)
  ;;;[1 1 1] Hide Clip in firearm mesh
  (Components|SkinnedMesh|HideBonebyName (Variables|Default|GetFirearmMesh) (GETFIREARMVALUES|GetReloadAttachBone) "PBO_None"))

(event EventSetInventoryItemAmmoCount
  (params (AmmoCount :type Integer) (Default :type Boolean))
  ;[1 1 1] INITIALIZE AMMO IN CLIP
  ;;[1 0.1179 0] [SERVER] BI FROM INVENTORY
  (if Default
    (bind _returnvalue (Utilities|GetDataTableRow "/Game/Blueprints/WeaponBase/DT_WeaponLibrary.DT_WeaponLibrary" (Variables|PUBLICSETTINGS|GetFirearmTag))
      (:then
        (Variables|COMMON|SetCurrentAmmoInClip (.MagazinSize (Utilities|Struct|BreakS_WeaponLibraryAmmoDesc (Utilities|Struct|BreakS_WeaponLibraryDesc _returnvalue))))))
    (else
      (Variables|COMMON|SetCurrentAmmoInClip AmmoCount))))

(event EventBIInventoryUpdateVisibilityMeshItem
  (params (NewVisibilityMode :type E_InventoryItemVisibilityMode%20Enum :default "NewEnumerator0"))
  ;[1 1 1] HANDLE UPDATE VISIBILITY MESH ITEM FOR OWNER
  ;;[1 0.1179 0] [CLIENT] BI FROM INVENTORY
  (CallFunction|ClientHandleUpdateVisibilityMeshItem NewVisibilityMode))

(fn ConstructionScript)

(fn GetinExtraReload
  (return (Variables|COMMON|GetInExtraReload)))

(fn UpdateAmmoonMainReload
  ;[1 1 1] Get Ammo Type
  (bind _returnvalue (Utilities|GetDataTableRow "/Game/Blueprints/WeaponBase/DT_WeaponLibrary.DT_WeaponLibrary" (Variables|PUBLICSETTINGS|GetFirearmTag))
    (:then
      (LocalVariables|Setloc_ammo_type (.AmmoType (Utilities|Struct|BreakS_WeaponLibraryAmmoDesc (.AmmoClip (Utilities|Struct|BreakS_WeaponLibraryDesc _returnvalue)))))
      (for _array_element (Default|GetInventoryResources (GETCOMPONENTS|GeInventorySystem))
        (LocalVariables|Setloc_step_res_type (.ResourceType (Utilities|Struct|BreakS_GL_InventoryResourceDesc _array_element)))
        (LocalVariables|Setloc_spet_ammo (.Amount (Utilities|Struct|BreakS_GL_InventoryResourceDesc _array_element)))
        (switch Utilities|FlowControl|Switch|SwitchonE_WeaponAmmoType (LocalVariables|Getloc_ammo_type)
          (:NewEnumerator0
            (if (Utilities|Enum|Equal(Enum) (LocalVariables|Getloc_step_res_type) "NewEnumerator0")
              (LocalVariables|Setloc_ammo_res_current (LocalVariables|Getloc_spet_ammo))
              (LocalVariables|Setloc_final_res (LocalVariables|Getloc_step_res_type))))
          (:NewEnumerator1
            (if (Utilities|Enum|Equal(Enum) (LocalVariables|Getloc_step_res_type) "NewEnumerator1")
              (LocalVariables|Setloc_ammo_res_current (LocalVariables|Getloc_spet_ammo))
              (LocalVariables|Setloc_final_res (LocalVariables|Getloc_step_res_type))))))
      ;[1 1 1] Calculation new ammo
      (LocalVariables|Setloc_AddAmmo (- (GETFIREARMVALUES|GetClipSize) (Variables|COMMON|GetCurrentAmmoInClip)))
      (if (> (LocalVariables|Getloc_AddAmmo) (LocalVariables|Getloc_ammo_res_current))
        (LocalVariables|Setloc_CurrentAmmoPull 0)
        (LocalVariables|Setloc_CurrentAmmoInClip (+ (LocalVariables|Getloc_ammo_res_current) (Variables|COMMON|GetCurrentAmmoInClip)))
        (else
          (LocalVariables|Setloc_CurrentAmmoPull (- (LocalVariables|Getloc_ammo_res_current) (LocalVariables|Getloc_AddAmmo)))
          (LocalVariables|Setloc_CurrentAmmoInClip (+ (LocalVariables|Getloc_AddAmmo) (Variables|COMMON|GetCurrentAmmoInClip)))))
      ;[1 1 1] Update Current Ammo in clip
      (Variables|COMMON|SetCurrentAmmoInClip (LocalVariables|Getloc_CurrentAmmoInClip))
      (return (LocalVariables|Getloc_final_res) (LocalVariables|Getloc_CurrentAmmoPull)))))

(fn GetClipSize
  (bind _returnvalue (Utilities|GetDataTableRow "/Game/Blueprints/WeaponBase/DT_WeaponLibrary.DT_WeaponLibrary" (Variables|PUBLICSETTINGS|GetFirearmTag))
    (:then
      (return (.MagazinSize (Utilities|Struct|BreakS_WeaponLibraryAmmoDesc (.AmmoClip (Utilities|Struct|BreakS_WeaponLibraryDesc _returnvalue))))))))

(fn GetUseExtraReload
  (bind _returnvalue (Utilities|GetDataTableRow "/Game/Blueprints/WeaponBase/DT_WeaponLibrary.DT_WeaponLibrary" (Variables|PUBLICSETTINGS|GetFirearmTag))
    (:then
      (return (.UseExtraReload (Utilities|Struct|BreakS_WeaponLibraryCommonDesc (.Common (Utilities|Struct|BreakS_WeaponLibraryDesc _returnvalue))))))))

(fn GetHoldingHandExtraReload
  (bind _returnvalue (Utilities|GetDataTableRow "/Game/Blueprints/WeaponBase/DT_WeaponLibrary.DT_WeaponLibrary" (Variables|PUBLICSETTINGS|GetFirearmTag))
    (:then
      (return (.HoldingHandExtraReload (Utilities|Struct|BreakS_WeaponLibraryCommonDesc (.Common (Utilities|Struct|BreakS_WeaponLibraryDesc _returnvalue))))))))

(fn GetAnimationID
  (bind _returnvalue (Utilities|GetDataTableRow "/Game/Blueprints/WeaponBase/DT_WeaponLibrary.DT_WeaponLibrary" (Variables|PUBLICSETTINGS|GetFirearmTag))
    (:then
      (return (.AnimationID (Utilities|Struct|BreakS_WeaponLibraryCommonDesc (.Common (Utilities|Struct|BreakS_WeaponLibraryDesc _returnvalue))))))))

(fn GetCurrentAmmoinClip
  (return (Variables|COMMON|GetCurrentAmmoInClip)))

(fn GeInventorySystem
  (bind _returnvalue (Components|GetOwner))
  (bind _asbp_base_pawn (Utilities|Casting|CastToBP_BasePawn _returnvalue))
  (bind _returnvalue_2 (Actor|GetComponentbyClass _asbp_base_pawn "/Game/Blueprints/InventorySystem/AC_InventorySystem.AC_InventorySystem_C"))
  (Utilities|IsValid _returnvalue_2
    (:Is%20Valid
      (return _returnvalue_2))))

(fn GeFirearmOwnerStateHandler
  (bind _returnvalue (Components|GetOwner))
  (bind _returnvalue_2 (Actor|GetComponentbyClass _returnvalue "/Game/Blueprints/WeaponSystem/AC_WeaponOwnerStateHandler.AC_WeaponOwnerStateHandler_C"))
  (Utilities|IsValid _returnvalue_2
    (:Is%20Valid
      (return _returnvalue_2))))

(fn GetMainReloadTime
  (bind _returnvalue (Utilities|GetDataTableRow "/Game/Blueprints/WeaponBase/DT_WeaponLibrary.DT_WeaponLibrary" (Variables|PUBLICSETTINGS|GetFirearmTag))
    (:then
      (return (.MainReloadTime (Utilities|Struct|BreakS_WeaponLibraryActionDesc (.Action (Utilities|Struct|BreakS_WeaponLibraryDesc _returnvalue))))))))

(fn GetShotDelay
  (bind _returnvalue (Utilities|GetDataTableRow "/Game/Blueprints/WeaponBase/DT_WeaponLibrary.DT_WeaponLibrary" (Variables|PUBLICSETTINGS|GetFirearmTag))
    (:then
      (return (/ 1.0 (/ (Math|Conversions|ToFloat(Integer) (.FireRate (Utilities|Struct|BreakS_WeaponLibraryShootDesc (.Shoot (Utilities|Struct|BreakS_WeaponLibraryDesc _returnvalue))))) 6e+01))))))

(fn GetShotTimePart
  (bind _returnvalue (Utilities|GetDataTableRow "/Game/Blueprints/WeaponBase/DT_WeaponLibrary.DT_WeaponLibrary" (Variables|PUBLICSETTINGS|GetFirearmTag))
    (:then
      (return (.ShotTimePart (Utilities|Struct|BreakS_WeaponLibraryShootDesc (.Shoot (Utilities|Struct|BreakS_WeaponLibraryDesc _returnvalue))))))))

(fn GetFiringMode
  (bind _returnvalue (Utilities|GetDataTableRow "/Game/Blueprints/WeaponBase/DT_WeaponLibrary.DT_WeaponLibrary" (Variables|PUBLICSETTINGS|GetFirearmTag))
    (:then
      (return (.FiringMode (Utilities|Struct|BreakS_WeaponLibraryShootDesc (.Shoot (Utilities|Struct|BreakS_WeaponLibraryDesc _returnvalue))))))))

(fn GetUseSimpleAnimMethod
  (bind _returnvalue (Utilities|GetDataTableRow "/Game/Blueprints/WeaponBase/DT_WeaponLibrary.DT_WeaponLibrary" (Variables|PUBLICSETTINGS|GetFirearmTag))
    (:then
      (return (.UseSimpleAnimMethod (Utilities|Struct|BreakS_WeaponLibraryCommonDesc (.Common (Utilities|Struct|BreakS_WeaponLibraryDesc _returnvalue))))))))

(fn GetReloadAttachBone
  (bind _returnvalue (Utilities|GetDataTableRow "/Game/Blueprints/WeaponBase/DT_WeaponLibrary.DT_WeaponLibrary" (Variables|PUBLICSETTINGS|GetFirearmTag))
    (:then
      (return (.ReloadAttachBone (Utilities|Struct|BreakS_WeaponLibraryCommonDesc (.Common (Utilities|Struct|BreakS_WeaponLibraryDesc _returnvalue))))))))

(fn GetFirearmIcon
  (bind _returnvalue (Utilities|GetDataTableRow "/Game/Blueprints/WeaponBase/DT_WeaponLibrary.DT_WeaponLibrary" (Variables|PUBLICSETTINGS|GetFirearmTag))
    (:then
      (return (.Icon (Utilities|Struct|BreakS_WeaponLibraryUIDesc (.UI (Utilities|Struct|BreakS_WeaponLibraryDesc _returnvalue))))))))

(fn GetFirearmName
  (bind _returnvalue (Utilities|GetDataTableRow "/Game/Blueprints/WeaponBase/DT_WeaponLibrary.DT_WeaponLibrary" (Variables|PUBLICSETTINGS|GetFirearmTag))
    (:then
      (return (.Name (Utilities|Struct|BreakS_WeaponibraryMiscDesc (.Misc (Utilities|Struct|BreakS_WeaponLibraryDesc _returnvalue))))))))

(fn GetAmmoType
  (bind _returnvalue (Utilities|GetDataTableRow "/Game/Blueprints/WeaponBase/DT_WeaponLibrary.DT_WeaponLibrary" (Variables|PUBLICSETTINGS|GetFirearmTag))
    (:then
      (return (Utilities|Struct|BreakS_WeaponLibraryAmmoDesc (Utilities|Struct|BreakS_WeaponLibraryDesc _returnvalue))))))

(fn GetAimTime
  (bind _returnvalue (Utilities|GetDataTableRow "/Game/Blueprints/WeaponBase/DT_WeaponLibrary.DT_WeaponLibrary" (Variables|PUBLICSETTINGS|GetFirearmTag))
    (:then
      (return (.AimDownSighttime (Utilities|Struct|BreakS_WeaponLibraryActionDesc (.Action (Utilities|Struct|BreakS_WeaponLibraryDesc _returnvalue))))))))

(fn GetFirearmIconWeaponModule
  (bind _returnvalue (Utilities|GetDataTableRow "/Game/Blueprints/WeaponBase/DT_WeaponLibrary.DT_WeaponLibrary" (Variables|PUBLICSETTINGS|GetFirearmTag))
    (:then
      (return (.HUDWeaponModule (Utilities|Struct|BreakS_WeaponLibraryUIDesc (.UI (Utilities|Struct|BreakS_WeaponLibraryDesc _returnvalue))))))))

(fn GetHoldingHandMainReload
  (bind _returnvalue (Utilities|GetDataTableRow "/Game/Blueprints/WeaponBase/DT_WeaponLibrary.DT_WeaponLibrary" (Variables|PUBLICSETTINGS|GetFirearmTag))
    (:then
      (return (.HoldingHandMainReload (Utilities|Struct|BreakS_WeaponLibraryCommonDesc (.Common (Utilities|Struct|BreakS_WeaponLibraryDesc _returnvalue))))))))

(fn GetInventoryType
  (bind _returnvalue (Utilities|GetDataTableRow "/Game/Blueprints/WeaponBase/DT_WeaponLibrary.DT_WeaponLibrary" (Variables|PUBLICSETTINGS|GetFirearmTag))
    (:then
      (return (.InventoryType (Utilities|Struct|BreakS_WeaponLibraryCommonDesc (.Common (Utilities|Struct|BreakS_WeaponLibraryDesc _returnvalue))))))))

(fn GetInventoryAmmoType
  (return (PUBLICGET|GetAmmoType)))

(fn GetInventoryItemAmmoCount
  (return (PUBLICGET|GetCurrentAmmoinClip)))

(fn GetInventoryItemIcon
  (return (PUBLICGET|GetFirearmIcon)))

(fn GetInventoryItemTitle
  (return (Utilities|Text|ToText(Name) (PUBLICGET|GetFirearmName))))

(fn GetInvetoryAttachments
  (return (Variables|COMMON|GetFirearm%20Attachments)))