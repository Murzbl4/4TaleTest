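; Third-person character pawn that connects its parent's firearm and state events to the weapon actor, animation Blueprint, VFX controller and camera.
; Server events multicast firearm attachment and animation, switching the holding hand around main reloads per weapon settings.
; Client events play hitscan VFX on the third-person weapon mesh.
; Main state changes select PlayerCameraTP presets by stance, gating aim presets on weapon state, and reattach the spring arm after a short delay.
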(event Custom|MulticastInitBaseAnimBP
  (params (FirearmTag :type Name))
  ;[1 1 1] HANDLE ATTACH & INITIALIZE FIREARM
  ;;[1 1 1] Initialize Base Anim BP
  ;;;[1 0.6824 0] TO ABP CHARACTER BASE
  (bind _asabp_character_base (Utilities|Casting|CastToABP_CharacterBase (Components|SkeletalMesh|GetAnimInstance (Variables|Character|GetMesh))))
  (Default|IntializeFirearmonAttaching _asabp_character_base FirearmTag))

(event Custom|ServerAttachCurrentFirearm
  ;[1 1 1] HANDLE ATTACH & INITIALIZE FIREARM
  ;;[1 1 1] ServerAttachCurrentFirearm
  (bind _asbp_weapon_actor_common (Utilities|Casting|CastToBP_WeaponActorCommon (Variables|COMMON|GetCurrentTPFirearm)))
  (if (Default|GetUseExtraReload _asbp_weapon_actor_common)
    (switch Utilities|FlowControl|Switch|SwitchonE_GL_WeaponHoldingHand (Default|GetHoldingHandExtraReload _asbp_weapon_actor_common)
      (:NewEnumerator0
        (CallFunction|MulticastAttachCurrentFirearmtoMesh true (Variables|COMMON|GetCurrentTPFirearm)))
      (:NewEnumerator1
        (CallFunction|MulticastAttachCurrentFirearmtoMesh false (Variables|COMMON|GetCurrentTPFirearm))))
    (else
      (CallFunction|MulticastAttachCurrentFirearmtoMesh true (Variables|COMMON|GetCurrentTPFirearm)))))

(event Custom|MulticastHandleChildFirearmEvent
  (params (FirearmEventType :type E_GL_WeaponEventType%20Enum :default "NewEnumerator0"))
  ;[1 1 1] HANDLE FIREARM EVENT
  ;;[1 1 1] Multicast Handle Firearm Event
  (bind _asabp_character_base (Utilities|Casting|CastToABP_CharacterBase (Components|SkeletalMesh|GetAnimInstance (Variables|Character|GetMesh))))
  (Default|HandleFirearmEvent _asabp_character_base FirearmEventType))

(event Custom|ServerHandleChildMainReloadStart
  ;[1 1 1] HANDLE FIREARM EVENT
  ;;[1 1 1] Server Main Reload Start
  (bind _asbp_weapon_actor_common (Utilities|Casting|CastToBP_WeaponActorCommon (Variables|COMMON|GetCurrentTPFirearm)))
  (CallFunction|MulticastAttachCurrentFirearmtoMesh (Utilities|Select :Index (Default|GetHoldingHandMainReload _asbp_weapon_actor_common) :NewEnumerator0 true :NewEnumerator1 false) (Variables|COMMON|GetCurrentTPFirearm)))

(event Custom|ServerHandleChildMainReloadFinish
  ;[1 1 1] HANDLE FIREARM EVENT
  ;;[1 1 1] Server Main Reload Finish
  (bind _asbp_weapon_actor_common (Utilities|Casting|CastToBP_WeaponActorCommon (Variables|COMMON|GetCurrentTPFirearm)))
  (if (Default|GetUseExtraReload _asbp_weapon_actor_common)
    (switch Utilities|FlowControl|Switch|SwitchonE_GL_WeaponHoldingHand (Default|GetHoldingHandExtraReload _asbp_weapon_actor_common)
      (:NewEnumerator0
        (CallFunction|MulticastAttachCurrentFirearmtoMesh true (Variables|COMMON|GetCurrentTPFirearm)))
      (:NewEnumerator1
        (CallFunction|MulticastAttachCurrentFirearmtoMesh false (Variables|COMMON|GetCurrentTPFirearm))))
    (else
      (CallFunction|MulticastAttachCurrentFirearmtoMesh true (Variables|COMMON|GetCurrentTPFirearm)))))

(event Custom|MulticastAttachCurrentFirearmToMesh
  (params (AttachToRightHand :type Boolean) (FirearmActor :type Actor%20Object%20Reference))
  ;[1 1 1] HANDLE ATTACH & INITIALIZE FIREARM
  ;;[1 1 1] MulticastAttachCurrentFirearmToMesh
  (Utilities|IsValid FirearmActor
    (:Is%20Valid
      (Transformation|AttachComponentToComponent FirearmActor (Variables|Character|GetMesh) (select AttachToRightHand (Variables|PRIVATESETTINGS|GetFirearmRHandAttachBone) (Variables|PRIVATESETTINGS|GetFirearmLHandAttachBone)) "SnapToTarget" "SnapToTarget" "KeepRelative" true))))

(event EventBeginPlay
  ;[1 1 1] EVENT BEGIN PLAY
  (|CallParentFunction)
  (CallFunction|ClientInitTPCameraAdvancedonSpawn))

(event EventServerClipEndFollow
  ;[1 1 1] HADNLE CLIP OBJ EVENTS
  ;;[1 1 1] Server Clip End Follow
  ;;;[0.1778 0 1] PARENT INPUT
  ;;;[1 0.6824 0] TO FIREARM ACTOR COMMON
  (bind _asbp_weapon_actor_common (Utilities|Casting|CastToBP_WeaponActorCommon (Variables|COMMON|GetCurrentTPFirearm)))
  (Default|ServerHandleClipEndFollowTP _asbp_weapon_actor_common))

(event EventServerClipinHand
  ;[1 1 1] HADNLE CLIP OBJ EVENTS
  ;;[1 1 1] Server Clip In Hand
  ;;;[0.1778 0 1] PARENT INPUT
  ;;;[1 0.6824 0] TO FIREARM ACTOR COMMON
  (bind _asbp_weapon_actor_common (Utilities|Casting|CastToBP_WeaponActorCommon (Variables|COMMON|GetCurrentTPFirearm)))
  (Default|ServerHandleClipinHandTP _asbp_weapon_actor_common))

(event EventClientHandleChildMultiTraceCreated
  (params (MultiTraceDesc :type Array%20of%20S%20Weapon%20Hit%20Scan%20Desc%20Structures))
  ;[1 1 1] HANDLE CREATED HITSCAN
  ;;[1 1 1] Multi Trace
  ;;;[0.1778 0 1] PARENT INPUT
  (bind _asbp_weapon_actor_common (Utilities|Casting|CastToBP_WeaponActorCommon (Variables|COMMON|GetCurrentTPFirearm)))
  ;;;[1 0.6824 0] TO FIREARM VFX CONTROLLER
  (Default|ClientStartPlayVFXonCreateMultiHitScanTP (CallFunction|GetFirearmVFXController) MultiTraceDesc (Variables|/Game/Blueprints/WeaponSystem/BP_WeaponActorCommon.BP_WeaponActorCommon_C|GetFirearmMesh _asbp_weapon_actor_common) false))

(event EventTick
  (params (DeltaSeconds :type Float%20%28single-precision%29))
  ;[1 1 1] EVENT TICK
  (|CallParentFunction DeltaSeconds))

(event EventServerChangedMainState
  (params (MainCharacterState :type E_CharacterMainState%20Enum :default "NewEnumerator0"))
  ;[1 1 1] HANDLE CHANGING MAIN STATE
  ;;[0.1778 0 1] PARENT INPUT EVENT
  (CallFunction|ClientDifineNewCameraPreset MainCharacterState)
  (CallFunction|ClientSwitchAttachignTPCamera MainCharacterState))

(event EventServerAttachFirearm
  (params (FirearmActor :type Actor%20Object%20Reference))
  ;[1 1 1] HANDLE ATTACH & INITIALIZE FIREARM
  ;;[1 1 1] Handle Attach Firearm
  ;;;[0.1778 0 1] PARENT INPUT
  (Variables|COMMON|SetCurrentTPFirearm FirearmActor)
  (bind _asbp_weapon_actor_common (Utilities|Casting|CastToBP_WeaponActorCommon (Variables|COMMON|GetCurrentTPFirearm)))
  (CallFunction|MulticastInitBaseAnimBP (Variables|/Game/Blueprints/WeaponSystem/BP_WeaponActorCommon.BP_WeaponActorCommon_C|GetFirearmTag _asbp_weapon_actor_common))
  (CallFunction|ServerAttachCurrentFirearm)
  ;;;[1 0.6824 0] TO PLAYER CAMERA TP
  (Default|ClientUpdateAimTime (Variables|Default|GetPlayerCameraTP) (Default|GetAimTime _asbp_weapon_actor_common)))

(event EventClientHandleChildSingleTraceCreated
  (params (SingleTraceDesc :type S%20Weapon%20Hit%20Scan%20Desc%20Structure))
  ;[1 1 1] HANDLE CREATED HITSCAN
  ;;[1 1 1] Single Trace
  ;;;[0.1778 0 1] PARENT INPUT
  (bind _asbp_weapon_actor_common (Utilities|Casting|CastToBP_WeaponActorCommon (Variables|COMMON|GetCurrentTPFirearm)))
  ;;;[1 0.6824 0] TO FIREARM VFX CONTROLLER
  (Default|ClientStartPlayVFXonCreateSingleHitScanTP (CallFunction|GetFirearmVFXController) SingleTraceDesc (Variables|/Game/Blueprints/WeaponSystem/BP_WeaponActorCommon.BP_WeaponActorCommon_C|GetFirearmMesh _asbp_weapon_actor_common) false))

(event EventServerHandleFirearmEvent
  (params (FirearmEventType :type E_GL_WeaponEventType%20Enum :default "NewEnumerator0"))
  ;[1 1 1] HANDLE FIREARM EVENT
  ;;[1 1 1] Server Handle Firearm Event
  ;;;[0.1778 0 1] PARENT INPUT
  (CallFunction|MulticastHandleChildFirearmEvent FirearmEventType)
  ;;;[1 0.6824 0] TO FIREARM ACTOR COMMON
  (bind _asbp_weapon_actor_common (Utilities|Casting|CastToBP_WeaponActorCommon (Variables|COMMON|GetCurrentTPFirearm)))
  (Default|ServerHandleTPFirearmEvent _asbp_weapon_actor_common FirearmEventType)
  (switch Utilities|FlowControl|Switch|SwitchonE_GL_WeaponEventType FirearmEventType
    (:NewEnumerator2
      (CallFunction|ServerHandleChildMainReloadStart))
    (:NewEnumerator3
      (CallFunction|ServerHandleChildMainReloadFinish))))

(event Custom|ClientTPCameraAdvancedChangePreset
  (params (NewCameraPreset :type Name))
  ;[1 1 1] Change Camera Preset
  ;;[1 0.6824 0] TO PLAYER CAMERA TP
  (Default|ClientOpenGateChange (Variables|Default|GetPlayerCameraTP))
  ;;[1 0.6824 0] TO PLAYER CAMERA TP
  (Default|ClientChangeCameraMode (Variables|Default|GetPlayerCameraTP) (Variables|Default|GetSpringArm) (Variables|Default|GetCamera) NewCameraPreset))

(event Custom|ClientDifineNewCameraPreset
  (params (MainCharacterState :type E_CharacterMainState%20Enum :default "NewEnumerator0"))
  ;[1 1 1] Difine New Camera Preset
  (switch Utilities|FlowControl|Switch|SwitchonE_CharacterMainState MainCharacterState
    (:NewEnumerator0
      (CallFunction|ClientTPCameraAdvancedChangePreset "StandIdle"))
    (:NewEnumerator12
      (CallFunction|ClientTPCameraAdvancedChangePreset "StandMove"))
    (:NewEnumerator1
      ;;[1 1 1] Check: Equip / Unarmed / Melee
      (if (not (Utilities|Enum|Equal(Enum) (CallFunction|GetCharacterWeaponState) "NewEnumerator0")) :!label _label
        (CallFunction|ClientTPCameraAdvancedChangePreset "StandAim")))
    (:NewEnumerator13
      (goto _label))
    (:NewEnumerator2
      (CallFunction|ClientTPCameraAdvancedChangePreset "CrouchIdle"))
    (:NewEnumerator14
      (CallFunction|ClientTPCameraAdvancedChangePreset "CrouchMove"))
    (:NewEnumerator3
      ;;[1 1 1] Check: Equip / Unarmed / Melee
      (if (not (Utilities|Enum|Equal(Enum) (CallFunction|GetCharacterWeaponState) "NewEnumerator0")) :!label _label_2
        (CallFunction|ClientTPCameraAdvancedChangePreset "CrouchAim")))
    (:NewEnumerator15
      (goto _label_2))
    (:NewEnumerator4
      (CallFunction|ClientTPCameraAdvancedChangePreset "ProneIdle"))
    (:NewEnumerator16
      (CallFunction|ClientTPCameraAdvancedChangePreset "ProneMove"))
    (:NewEnumerator5
      ;;[1 1 1] Check: Equip / Unarmed / Melee
      (if (not (Utilities|Enum|Equal(Enum) (CallFunction|GetCharacterWeaponState) "NewEnumerator0")) :!label _label_3
        (CallFunction|ClientTPCameraAdvancedChangePreset "ProneAim")))
    (:NewEnumerator17
      (goto _label_3))
    (:NewEnumerator6
      (CallFunction|ClientTPCameraAdvancedChangePreset "Sprint"))
    (:NewEnumerator11
      (CallFunction|ClientTPCameraAdvancedChangePreset "Dead"))))

(event Custom|ClientSwitchAttachignTPCamera
  (params (CharacterState :type E_CharacterMainState%20Enum :default "NewEnumerator0"))
  ;[1 1 1] Switch Attacing TP Camera
  (Utilities|FlowControl|Delay 0.3)
  (Transformation|AttachComponentToComponent (Variables|Default|GetSpringArm) (Variables|Character|GetMesh) "VB TPCamRootPoint" "KeepRelative" "KeepRelative" "KeepRelative" true)
  (Transformation|SetRelativeLocation (Variables|Default|GetSpringArm) "0, 0, 0" false false))

(event Custom|ClientInitTPCameraAdvancedOnSpawn
  ;[1 1 1] Init Camera On Spawn
  (Utilities|IsValid (Variables|Default|GetPlayerCameraTP)
    (:Is%20Valid
      (Utilities|IsValid (Variables|Default|GetSpringArm)
        (:Is%20Valid
          (Utilities|IsValid (Variables|Default|GetCamera)
            (:Is%20Valid
              ;;[1 0.6824 0] TO PLAYER CAMERA TP
              (Default|ClientSetStartCameraMode (Variables|Default|GetPlayerCameraTP) (Variables|Default|GetSpringArm) (Variables|Default|GetCamera) "StandIdle" true))))))))

(fn ConstructionScript
  (|CallParentFunction))